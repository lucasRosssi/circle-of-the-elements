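; BP_EnemyBase is an enemy Blueprint that handles summon, dissolve and target-facing presentation.
; On summon, a timeline drives uniform mesh scale.
; Two dissolve events run separate timelines, one named for the weapon, that drive the "Dissolve" scalar on a passed-in dynamic material, using a separate track for Minion character types.
; UpdateFacingTarget writes the given location to the "FacingTarget" Motion Warping target.
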(event EventOnSummoned
  (bind _scaletrack (Timeline|SummonTimeline Play)
    (:Update
      (Transformation|SetRelativeScale3D (Variables|Character|GetMesh) (Math|Vector|MakeVector _scaletrack _scaletrack _scaletrack)))))

(event EventStartDissolveTimeline
  (params (DynamicMaterialInstance :type Material%20Instance%20Dynamic%20Object%20Reference))
  (bind (_direction _dissolvetrack _miniondissolvetrack) (Timeline|DissolveTimeline Play)
    (:Update
      (if (Utilities|Enum|Equal(Enum) (Variables|Default|GetCharacterType) "ECT_Minion")
        (Rendering|Material|SetScalarParameterValue DynamicMaterialInstance "Dissolve" _miniondissolvetrack :!class /Script/Engine.MaterialInstanceDynamic)
        (else
          (Rendering|Material|SetScalarParameterValue DynamicMaterialInstance "Dissolve" _dissolvetrack :!class /Script/Engine.MaterialInstanceDynamic))))))

(event EventStartWeaponDissolveTimeline
  (params (DynamicMaterialInstance :type Material%20Instance%20Dynamic%20Object%20Reference))
  (bind (_direction _dissolvetrack _miniondissolvetrack) (Timeline|WeaponDissolveTimeline Play)
    (:Update
      (if (Utilities|Enum|Equal(Enum) (Variables|Default|GetCharacterType) "ECT_Minion")
        (Rendering|Material|SetScalarParameterValue DynamicMaterialInstance "Dissolve" _miniondissolvetrack :!class /Script/Engine.MaterialInstanceDynamic)
        (else
          (Rendering|Material|SetScalarParameterValue DynamicMaterialInstance "Dissolve" _dissolvetrack :!class /Script/Engine.MaterialInstanceDynamic))))))

(event EventUpdateFacingTarget
  (params (TargetLocation :type Vector%20%28by%20ref%29 :default "0, 0, 0"))
  (Class|MotionWarpingComponent|AddorUpdateWarpTargetfromLocation (Variables|Default|GetMotionWarping) "FacingTarget" TargetLocation))

(fn ConstructionScript)