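; BP_Gate is an interactable gate trigger that sends the hero to the bottom-left entrance of the Crystal Cave region once an encounter finishes.
; It unlocks when the AuraGameMode's encounter-finished delegate fires.
; Its Box overlap tracks hero range and binds or unbinds the player controller's interact action.
; Interacting while in range and unlocked calls GoToLocation on the game mode, with a hard-coded destination and debug prints throughout.
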(event OnComponentBeginOverlap(Box)
  (params (OverlappedComponent :type Primitive%20Component%20Object%20Reference) (OtherActor :type Actor%20Object%20Reference) (OtherComp :type Primitive%20Component%20Object%20Reference) (OtherBodyIndex :type Integer) (bFromSweep :type Boolean) (SweepResult :type Hit%20Result%20Structure%20%28by%20ref%29))
  (bind _asaura_hero (Utilities|Casting|CastToAuraHero OtherActor))
  (Variables|Default|SetPlayerInRange true)
  (Development|PrintString "Player in range")
  (bind _asaura_player_controller (Utilities|Casting|CastToAuraPlayerController (Pawn|GetController _asaura_hero)))
  (EventDispatchers|BindEventtoInteractActionTriggered _asaura_player_controller (delegate Custom|OnInteract_Event)))

(event OnComponentEndOverlap(Box)
  (params (OverlappedComponent :type Primitive%20Component%20Object%20Reference) (OtherActor :type Actor%20Object%20Reference) (OtherComp :type Primitive%20Component%20Object%20Reference) (OtherBodyIndex :type Integer))
  (bind _asaura_hero (Utilities|Casting|CastToAuraHero OtherActor))
  (Variables|Default|SetPlayerInRange false)
  (Development|PrintString "Player out of range")
  (bind _asaura_player_controller (Utilities|Casting|CastToAuraPlayerController (Pawn|GetController _asaura_hero)))
  (EventDispatchers|UnbindEventfromInteractActionTriggered _asaura_player_controller (delegate Custom|OnInteract_Event)))

(event Custom|OnEncounterFinishedDelegate_Event
  (Variables|Default|SetCanBeActivated true)
  (Development|PrintString "Can use Gate"))

(event Custom|OnInteract_Event
  (Development|PrintString "E pressed")
  (if (and (Variables|Default|GetPlayerInRange) (Variables|Default|GetCanBeActivated))
    (bind _asaura_game_mode_base (Utilities|Casting|CastToAuraGameModeBase (Game|GetGameMode)))
    (Class|AuraGameModeBase|GotoLocation _asaura_game_mode_base "CrystalCave" "BottomLeft")))

(event EventBeginPlay
  (bind _asaura_game_mode_base (Utilities|Casting|CastToAuraGameModeBase (Game|GetGameMode)))
  (EventDispatchers|AssignOnEncounterFinishedDelegate _asaura_game_mode_base (delegate Custom|OnEncounterFinishedDelegate_Event))
  (Development|PrintString "Event bound"))

(fn ConstructionScript)