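; Interactable crystal cave gate that takes the player out of the current location.
; On interaction it disables the player controller, sinks the gate mesh, then resets the hero's rotation and plays an enter-gate montage.
; Shortly after the montage starts, the overlay widget controller begins a screen transition.
; When the montage completes, the game mode exits the location using the next gate position.
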(event EventOnInteracted
  (params (InInstigator :type Actor%20Object%20Reference))
  (bind _asaura_player_controller (Utilities|Casting|CastToAuraPlayerController (Game|GetPlayerController 0)))
  (Class|AuraPlayerController|DisableController _asaura_player_controller)
  (Components|MoveComponentTo (Variables|Default|GetGateMesh) "0.000000,0.000000,-600.000000" "0, 0, 0" false false 1.0 false)
  (bind _asaura_hero (Utilities|Casting|CastToAuraHero (Game|GetPlayerCharacter 0)))
  (Transformation|SetActorRotation _asaura_hero)
  (Animation|Montage|PlayMontage (Variables|/Script/Engine.Character|GetMesh _asaura_hero) "/Game/Assets/Characters/Aura/Animations/AM_EnterGate.AM_EnterGate"
    (:then
      (Utilities|FlowControl|Delay 0.5)
      (Class|OverlayWidgetController|StartTransition (Class|AuraAbilitySystemLibrary|GetOverlayWidgetController)))
    (:OnCompleted
      (Class|AuraGameModeBase|ExitLocation (Class|Interactable|GetAuraGameMode) (Variables|Default|GetNextGatePosition)))))

(fn ConstructionScript)