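; BP_CrystalCaveGate is a Crystal Cave gate interactable that opens or blocks a passage through two blocker meshes.
; Its active-toggle event hides both meshes and disables their collision when active, and shows them with query-only collision when inactive.
; The construction script only calls the parent's, and BeginPlay, overlap and Tick are unused.
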(event EventBeginPlay)

(event Collision|EventActorBeginOverlap
  (params (OtherActor :type Actor%20Object%20Reference)))

(event EventTick
  (params (DeltaSeconds :type Float%20%28single-precision%29)))

(event EventOnActiveToggle
  (params (bIsActive :type Boolean))
  (bind _blockedmesh1 (Variables|Default|GetBlockedMesh1))
  (bind _blockedmesh2 (Variables|Default|GetBlockedMesh2))
  (bind _blockedmesh1_2 (Variables|Default|GetBlockedMesh1))
  (bind _blockedmesh2_2 (Variables|Default|GetBlockedMesh2))
  (if bIsActive
    (Rendering|SetVisibility _blockedmesh1_2 false false)
    (Collision|SetCollisionEnabled _blockedmesh1_2 "NoCollision")
    (Rendering|SetVisibility _blockedmesh2_2 false false)
    (Collision|SetCollisionEnabled _blockedmesh2_2 "NoCollision")
    (else
      (Rendering|SetVisibility _blockedmesh1 true false)
      (Collision|SetCollisionEnabled _blockedmesh1 "QueryOnly")
      (Rendering|SetVisibility _blockedmesh2 true false)
      (Collision|SetCollisionEnabled _blockedmesh2 "QueryOnly"))))

(fn ConstructionScript
  (|CallParentFunction))