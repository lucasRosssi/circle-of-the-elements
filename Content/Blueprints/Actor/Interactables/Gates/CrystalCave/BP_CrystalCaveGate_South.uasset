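; South crystal cave gate interactable, a child Blueprint that relies on its parent for its core behavior.
; It extends the parent's active-toggle event, hiding the BlockedMesh3 component when the gate becomes active.
; Deactivation does not restore that mesh here, and the construction script only calls the parent.
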(event EventBeginPlay
  (|CallParentFunction) ; This node is disabled and will not be called.\nDrag off pins to build functionality.
)

(event Collision|EventActorBeginOverlap
  (params (OtherActor :type Actor%20Object%20Reference))
  (|CallParentFunction OtherActor) ; This node is disabled and will not be called.\nDrag off pins to build functionality.
)

(event EventTick
  (params (DeltaSeconds :type Float%20%28single-precision%29))
  (|CallParentFunction DeltaSeconds) ; This node is disabled and will not be called.\nDrag off pins to build functionality.
)

(event EventOnActiveToggle
  (params (bIsActive :type Boolean))
  (|CallParentFunction bIsActive)
  (if bIsActive
    (Rendering|SetVisibility (Variables|Default|GetBlockedMesh3) false false)))

(fn ConstructionScript
  (|CallParentFunction))