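; Crystal cave east gate, a child Blueprint that sets up its wall meshes according to the gate's active state.
; It extends the parent's OnActiveToggle event, passing the state to HandleGateMeshes.
; That function hides and removes collision from SouthWall meshes 2 and 4 when active, or 1 and 3 when inactive.
; It only disables meshes and never restores their visibility or collision.
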(event EventBeginPlay
  (|CallParentFunction) ; This node is disabled and will not be called.\nDrag off pins to build functionality.
)

(event Collision|EventActorBeginOverlap
  (params (OtherActor :type Actor%20Object%20Reference))
  (|CallParentFunction OtherActor) ; This node is disabled and will not be called.\nDrag off pins to build functionality.
)

(event EventTick
  (params (DeltaSeconds :type Float%20%28single-precision%29))
  (|CallParentFunction DeltaSeconds) ; This node is disabled and will not be called.\nDrag off pins to build functionality.
)

(event EventOnActiveToggle
  (params (bIsActive :type Boolean))
  (|CallParentFunction bIsActive)
  (CallFunction|HandleGateMeshes bIsActive))

(fn ConstructionScript
  (|CallParentFunction))

(fn HandleGateMeshes
  (params (IsActive :type Boolean))
  (bind _southwallmesh2 (Variables|Default|GetSouthWallMesh2))
  (bind _southwallmesh4 (Variables|Default|GetSouthWallMesh4))
  (bind _southwallmesh1 (Variables|Default|GetSouthWallMesh1))
  (bind _southwallmesh3 (Variables|Default|GetSouthWallMesh3))
  (if IsActive
    (Rendering|SetVisibility _southwallmesh2 false false)
    (Collision|SetCollisionEnabled _southwallmesh2 "NoCollision")
    (Rendering|SetVisibility _southwallmesh4 false false)
    (Collision|SetCollisionEnabled _southwallmesh4 "NoCollision")
    (else
      (Rendering|SetVisibility _southwallmesh1 false false)
      (Collision|SetCollisionEnabled _southwallmesh1 "NoCollision")
      (Rendering|SetVisibility _southwallmesh3 false false)
      (Collision|SetCollisionEnabled _southwallmesh3 "NoCollision"))))