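; Base interactable gate that carries the hero out of the current location and displays its assigned reward on a globe widget.
; On interaction it disables the controller, lowers the gate mesh and rotates the hero using a lookup keyed by next gate position.
; The enter-gate montage runs alongside a delayed overlay transition, and its completion tells the location manager to exit toward that position.
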(event EventRewardAssigned
  (bind _aswbp_reward_globe (Utilities|Casting|CastToWBP_RewardGlobe (UserInterface|GetWidget (Variables|Default|GetRewardWidget))))
  (Default|SetReward _aswbp_reward_globe (Variables|Default|GetRewardTag)))

(event EventOnInteracted
  (params (InstigatorController :type Aura%20Player%20Controller%20Object%20Reference))
  (Class|AuraPlayerController|DisableController InstigatorController)
  (Components|MoveComponentTo (Variables|Default|GetGateMesh) "0.000000,0.000000,-600.000000" "0, 0, 0" false false 1.0 false)
  (bind _asaura_hero (Utilities|Casting|CastToAuraHero (Pawn|GetControlledPawn InstigatorController)))
  (Transformation|SetActorRotation _asaura_hero (.Value (Utilities|Map|Find (Variables|Default|GetNextGatePositionToRotation) (Variables|Default|GetNextGatePosition))))
  (Animation|Montage|PlayMontage (Variables|/Script/Engine.Character|GetMesh _asaura_hero) "/Game/Assets/Characters/Aura/Animations/AM_EnterGate.AM_EnterGate"
    (:then
      (Utilities|FlowControl|Delay 0.5)
      (Class|OverlayWidgetController|StartTransition (Class|AuraAbilitySystemLibrary|GetOverlayWidgetController)))
    (:OnCompleted
      (Class|LocationManager|ExitLocation (Class|AuraSystemsLibrary|GetLocationManager) (Variables|Default|GetNextGatePosition)))))

(fn ConstructionScript)