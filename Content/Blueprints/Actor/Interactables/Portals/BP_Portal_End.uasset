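; End portal actor that lets the player end the match once combat in its area is finished.
; On BeginPlay it subscribes to the combat manager's combat-finished delegate.
; When that delegate reports a matching area name, it enables its interact component and activates its Niagara effect.
; Interacting then calls EndMatch on the match manager with a true flag.
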(event Custom|OnCombatFinishedDelegate_Event
  (params (AreaName :type Name))
  (if (== AreaName (Variables|Default|GetAreaName))
    (Class|InteractComponent|EnableInteraction (Variables|Default|GetInteractComponent))
    (Components|Activation|Activate (Variables|Default|GetNiagara) false)))

(event EventBeginPlay
  (EventDispatchers|AssignOnCombatFinishedDelegate (Class|AuraSystemsLibrary|GetCombatManager) (delegate Custom|OnCombatFinishedDelegate_Event)))

(event EventInteract
  (params (Controller :type Controller%20Object%20Reference))
  (Class|MatchManager|EndMatch (Class|AuraSystemsLibrary|GetMatchManager) true))

(fn ConstructionScript)