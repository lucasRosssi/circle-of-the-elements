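; Base interactable gate that takes the player's Aura hero out of the current location.
; On interaction it disables the player controller, sinks the gate mesh over a second, zeroes the hero's rotation and plays an enter-gate montage.
; Shortly into the montage the overlay widget controller starts a screen transition, and on montage completion the game mode exits the location using the next gate position.
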(event EventOnInteracted
  (params (InstigatorController :type Controller%20Object%20Reference))
  (bind _asaura_player_controller (Utilities|Casting|CastToAuraPlayerController InstigatorController))
  (Class|AuraPlayerController|DisableController _asaura_player_controller)
  (Components|MoveComponentTo (Variables|Default|GetGateMesh) "0.000000,0.000000,-600.000000" "0, 0, 0" false false 1.0 false)
  (bind _asaura_hero (Utilities|Casting|CastToAuraHero (Pawn|GetControlledPawn _asaura_player_controller)))
  (Transformation|SetActorRotation _asaura_hero)
  (Animation|Montage|PlayMontage (Variables|/Script/Engine.Character|GetMesh _asaura_hero) "/Game/Assets/Characters/Aura/Animations/AM_EnterGate.AM_EnterGate"
    (:then
      (Utilities|FlowControl|Delay 0.5)
      (Class|OverlayWidgetController|StartTransition (Class|AuraAbilitySystemLibrary|GetOverlayWidgetController)))
    (:OnCompleted
      (Class|AuraGameModeBase|ExitLocation (Class|Interactable|GetAuraGameMode) (Variables|Default|GetNextGatePosition)))))

(fn ConstructionScript)