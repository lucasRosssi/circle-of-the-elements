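; Base fire prop for environments that changes its look to match its element.
; When the element is set, it looks up the element tag in maps to swap the Niagara effect and light color.
; From BeginPlay, MoveLightOrigin endlessly eases the light to small random offsets around its starting position over short random durations, mostly vertically, to mimic flame flicker.
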(event EventOnElementSet
  (Class|NiagaraComponent|SetAsset (Variables|Default|GetNiagara) (.Value (Utilities|Map|Find (Variables|Default|GetElementNiagara) (Variables|Default|GetElementTag))) true)
  (Rendering|Components|Light|SetLightColor (Variables|Default|GetLight) (.Value (Utilities|Map|Find (Variables|Default|GetElementColor) (Variables|Default|GetElementTag))) true))

(event EventBeginPlay
  (Utilities|MoveLightOrigin))

(fn ConstructionScript)