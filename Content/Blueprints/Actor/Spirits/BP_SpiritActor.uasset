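; BP_SpiritActor is a spirit actor whose Spirit component, exposed through a Niagara getter, gently bobs up and down.
; Every tick, Float advances a wrapping timer and offsets the component's relative Z from its initial location by an amplitude-scaled sine wave.
; While the spirit is using an ability or is hijacked, the timer pauses and the component stays at its initial location.
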(event EventBeginPlay)

(event EventTick
  (params (DeltaSeconds :type Float%20%28single-precision%29))
  (CallFunction|Float DeltaSeconds))

(fn ConstructionScript)

(fn UpdateTime
  (params (DeltaTime :type Float%20%28double-precision%29))
  (bind _output_get (Variables|Default|SetTime (+ DeltaTime (Variables|Default|GetTime))))
  (if (> _output_get (* 2.0 (Math|Trig|GetPI)))
    (Variables|Default|SetTime 0.0)))

(fn SinOfTime
  (return (* (Math|Trig|Sin(Radians) (Variables|Default|GetTime)) (Variables|Default|GetAmplitude))))

(fn GetSpiritNiagara
  (return (Variables|Default|GetSpirit)))

(fn Float
  (params (DeltaTime :type Float%20%28double-precision%29))
  (if (or (Class|SpiritActor|IsUsingAbility) (Class|SpiritActor|IsHijacked))
    (Transformation|SetRelativeLocation (Variables|Default|GetSpirit) (Variables|Default|GetSpiritInitialLocation) false false)
    (else
      (CallFunction|UpdateTime DeltaTime)
      (Transformation|SetRelativeLocation (Variables|Default|GetSpirit) (+ (Variables|Default|GetSpiritInitialLocation) (Math|Vector|MakeVector 0.0 0.0 (CallFunction|SinOfTime))) false false))))