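; BP_AuraHero is the Blueprint for the Aura hero character, with BeginPlay only calling its parent.
; A DebugDirectionInput function, not called within this graph, draws an arrow along the Aura player controller's InputDirection and prints that vector on screen.
; Custom depth stencil setup on the mesh sits disconnected and never runs, and the construction script is empty.
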(event EventBeginPlay
  (|CallParentFunction))

(fn ConstructionScript)

(fn DebugDirectionInput
  (bind _asbp_aura_player_controller (Utilities|Casting|CastToBP_AuraPlayerController (Game|GetPlayerController 0)))
  (Rendering|Debug|DrawDebugArrow (Transformation|GetActorLocation) (+ (* (Variables|/Script/Aura.AuraPlayerController|GetInputDirection _asbp_aura_player_controller) 1.5e+02) (Transformation|GetActorLocation)) 2e+02 "(R=0.000000,G=1.000000,B=0.006852,A=1.000000)" 0.0 3.0)
  (Development|PrintString (Utilities|String|ToString(Vector) (Variables|/Script/Aura.AuraPlayerController|GetInputDirection _asbp_aura_player_controller)) true false "(R=0.000000,G=0.660000,B=1.000000,A=1.000000)" 1.0 "1"))