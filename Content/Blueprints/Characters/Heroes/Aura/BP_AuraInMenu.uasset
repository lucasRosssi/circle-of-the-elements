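; BP_AuraInMenu is the menu version of the Aura hero, with an energy ball that bobs gently up and down.
; BeginPlay caches the ball's world location and slows the ball with a custom time dilation.
; Each tick accumulates time, resets it after a full two-pi cycle, and offsets the ball's height from that cached location by an amplitude-scaled sine.
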(event EventTick
  (params (DeltaSeconds :type Float%20%28single-precision%29))
  (|CallParentFunction DeltaSeconds)
  (CallFunction|UpdateTime DeltaSeconds)
  (Transformation|SetWorldLocation (Variables|Default|GetEnergyBall) (+ (Variables|Default|GetEnergyBallInitialLocation) (Math|Vector|MakeVector 0.0 0.0 (CallFunction|SinOfTime))) false false))

(event EventBeginPlay
  (|CallParentFunction)
  (Variables|Default|SetEnergyBallInitialLocation (Transformation|GetWorldLocation (Variables|Default|GetEnergyBall)))
  (Class|NiagaraComponent|SetCustomTimeDilation (Variables|Default|GetEnergyBall) 0.75))

(fn ConstructionScript
  (|CallParentFunction))

(fn UpdateTime
  (params (DeltaTime :type Float%20%28double-precision%29))
  (bind _output_get (Variables|Default|SetTime (+ DeltaTime (Variables|Default|GetTime))))
  (if (> _output_get (* 2.0 (Math|Trig|GetPI)))
    (Variables|Default|SetTime 0.0)))

(fn SinOfTime
  (return (* (Math|Trig|Sin(Radians) (Variables|Default|GetTime)) (Variables|Default|GetAmplitude))))