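; BP_AuraGameMode is a game mode that spawns the player's selected hero when play begins.
; It reads CurrentHeroClass from BP_AuraGameInstance, spawns that class at a found player start, nudging it clear of collisions but always spawning.
; Player controller 0 then possesses the hero and has its tick enabled, and the pawn is added uniquely to the Players list.
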(event EventBeginPlay
  (bind _returnvalue (Game|GetPlayerController 0))
  (bind _asbp_aura_game_instance (Utilities|Casting|CastToBP_AuraGameInstance (Game|GetGameInstance)))
  (bind _returnvalue_2 (Game|SpawnActorfromClass (Variables|/Game/Blueprints/Game/BP_AuraGameInstance.BP_AuraGameInstance_C|GetCurrentHeroClass _asbp_aura_game_instance) (Transformation|GetActorTransform (Class|GameModeBase|FindPlayerStart _returnvalue)) "AdjustIfPossibleButAlwaysSpawn" "MultiplyWithRoot" 0 0))
  (Pawn|Possess _returnvalue _returnvalue_2)
  (Actor|Tick|SetActorTickEnabled _returnvalue true)
  (Utilities|Array|AddUnique (Variables|Default|GetPlayers) (Game|Player|GetPlayerPawn 0)))

(fn ConstructionScript)