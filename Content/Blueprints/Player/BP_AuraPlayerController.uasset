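; Player controller Blueprint for the Aura player, handling camera occlusion fading, gamepad detection and menu opening.
; Occlusion changes drive a timeline that writes OcclusionSize into a material parameter collection, reversing at half speed when clear.
; UIManager events create the skill selection and character menu widgets and hand them back to UIManager.
; It also attaches the audio listener to the pawn, and the G key teleports the pawn to a player start.
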(event OpenSkillSelectionMenu(UIManager)
  (params (ElementTag :type Gameplay%20Tag%20Structure%20%28by%20ref%29))
  (CallFunction|OpenSkillSelectionMenu ElementTag))

(event OpenCharacterMenu(UIManager)
  (params (ActiveTabIndex :type Integer))
  (CallFunction|OpenCharacterMenu ActiveTabIndex))

(event EventBeginPlay
  (Class|PlayerController|SetAudioListenerOverride (Variables|/Script/Engine.Actor|GetRootComponent (Pawn|GetControlledPawn)) "0, 0, 0" "0, 0, 0"))

(event EventOnOcclusionChange
  (params (bIsOccluding :type Boolean))
  (if bIsOccluding
    (Components|Timeline|SetPlayRate (Variables|Default|GetFadeTimeline) 1.0)
    (bind _occlusionsize (Timeline|FadeTimeline Play)
      (:Update
        (Rendering|Material|SetScalarParameterValue "/Game/Assets/Materials/CameraOcclusion/MPC_CameraOcclusionMask.MPC_CameraOcclusionMask" "OcclusionSize" _occlusionsize :!class /Script/Engine.KismetMaterialLibrary)))
    (else
      (Components|Timeline|SetPlayRate (Variables|Default|GetFadeTimeline) 0.5)
      (Timeline|FadeTimeline Reverse))))

(event Input|KeyboardEvents|AnyKey
  (params (Key :type Key%20Structure :default "None"))
  (bind _returnvalue (Class|KismetInputLibrary|KeyIsGamepadKey Key))
  (:Pressed
    (if (!= _returnvalue (Variables|Default|GetbUsingGamepad))
      (Class|AuraPlayerController|ChangeUsingGamepad _returnvalue))))

(event Input|KeyboardEvents|G
  (params (Key :type Key%20Structure :default "None"))
  (:Pressed
    (Transformation|SetActorLocation (Pawn|GetControlledPawn) (Transformation|GetActorLocation (Class|GameModeBase|FindPlayerStart (Game|GetGameMode) self)) false true)))

(fn ConstructionScript)

(fn OpenSkillSelectionMenu
  (params (ElementTag :type Gameplay%20Tag%20Structure))
  (bind _returnvalue (UserInterface|CreateWidget "/Game/Blueprints/UI/RewardMenus/WBP_SkillSelectionMenu.WBP_SkillSelectionMenu_C" self))
  (Variables|/Game/Blueprints/UI/RewardMenus/WBP_SkillSelectionMenu.WBP_SkillSelectionMenu_C|SetElementTag _returnvalue ElementTag)
  (Class|UIManager|OpenWidget (Variables|Default|GetUIManager) _returnvalue))

(fn OpenCharacterMenu
  (params (InputPin :type Integer))
  (bind _returnvalue (UserInterface|CreateWidget "/Game/Blueprints/UI/CharacterMenu/WBP_CharacterMenu.WBP_CharacterMenu_C" self))
  (Default|ActivateTab _returnvalue InputPin)
  (Class|UIManager|OpenWidget (Variables|Default|GetUIManager) _returnvalue))