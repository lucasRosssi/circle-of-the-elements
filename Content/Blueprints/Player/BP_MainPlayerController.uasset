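; Main player controller that handles audio listening, input device detection and camera occlusion masking.
; On BeginPlay it attaches the audio listener override to the controlled pawn's root component.
; Any key press updates the gamepad-usage state when the input device type changes.
; Occlusion changes drive a timeline that writes the mask size to a Material Parameter Collection, reversing at half speed when occlusion ends.
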(event EventBeginPlay
  (Class|PlayerController|SetAudioListenerOverride (Variables|/Script/Engine.Actor|GetRootComponent (Pawn|GetControlledPawn)) "0, 0, 0" "0, 0, 0"))

(event EventOnOcclusionChange
  (params (bIsOccluding :type Boolean))
  (if bIsOccluding
    (Components|Timeline|SetPlayRate (Variables|Default|GetFadeTimeline) 1.0)
    (bind _occlusionsize (Timeline|FadeTimeline Play)
      (:Update
        (Rendering|Material|SetScalarParameterValue "/Game/Assets/Materials/CameraOcclusion/MPC_CameraOcclusionMask.MPC_CameraOcclusionMask" "OcclusionSize" _occlusionsize :!class /Script/Engine.KismetMaterialLibrary)))
    (else
      (Components|Timeline|SetPlayRate (Variables|Default|GetFadeTimeline) 0.5)
      (Timeline|FadeTimeline Reverse))))

(event Input|KeyboardEvents|AnyKey
  (params (Key :type Key%20Structure))
  (bind _returnvalue (Class|KismetInputLibrary|KeyIsGamepadKey Key))
  (:Pressed
    (if (!= _returnvalue (Variables|Default|GetbUsingGamepad))
      (Class|MainPlayerController|ChangeUsingGamepad _returnvalue))))

(fn ConstructionScript)