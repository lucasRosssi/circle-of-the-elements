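; Melee attack gameplay ability that plays a montage and damages nearby enemies, for player or AI users.
; It first faces the cursor hit (PlayerAbility) or combat target.
; On each Event.Montage.AttackScan event, it scans a radius around an ability socket, damaging living, non-invulnerable enemies with hit sounds, then fires a gameplay cue if TargetWasHit.
; It ends on montage completion, interruption, cancellation or, optionally, blend out.
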(event Ability|EventActivateAbility
  (bind _returnvalue (Ability|GetAvatarActorfromActorInfo))
  (bind _returnvalue_2 (Ability|GetAvatarActorfromActorInfo))
  (bind _returnvalue_3 (Ability|GetAvatarActorfromActorInfo))
  (if (Variables|Default|GetPlayerAbility)
    (bind _datahandle (|TargetDataUnderMouse)
      (:ValidData
        (Class|CombatInterface|UpdateFacingTarget(Message) (Ability|GetAvatarActorfromActorInfo) (.Location (Collision|BreakHitResult (Ability|TargetData|GetHitResultfromTargetData _datahandle))))))
    (else
      (Variables|Default|SetTargetWasHit false)
      (bind _returnvalue_4 (Class|CombatInterface|GetCombatTarget(Message) _returnvalue))
      (Class|CombatInterface|UpdateFacingTarget(Message) _returnvalue (Transformation|GetActorLocation _returnvalue_4))))
  (|PlayMontageandWaitProxy "None" (Variables|Default|GetMontage%20to%20Play) (Variables|Default|GetMontage%20Play%20Rate) "None" true (Variables|Default|GetAnim%20Root%20Motion%20Translation%20Scale) 0.0
    (:then
      (Ability|Tasks|WaitGameplayEvent "(TagName=\"Event.Montage.AttackScan\")" 0
        (:EventReceived
          (bind _returnvalue_5 (Class|CombatInterface|GetAbilitySocketLocation(Message) _returnvalue_2 (Variables|Default|GetAbilitySocketName) (Variables|Default|GetAbilitySocketInWeapon)))
          (bind _outoverlappingactors (Class|AuraAbilitySystemLibrary|GetAliveCharactersWithinRadius _returnvalue_2 (Utilities|Array|MakeArray _returnvalue_2) (Variables|Default|GetMeleeHitScanRadius) _returnvalue_5))
          (for _array_element _outoverlappingactors
            (CallFunction|HandleTargetHit _array_element))
          (if (Variables|Default|GetTargetWasHit)
            (Class|GameplayAbility|ExecuteGameplayCuewithParams (Variables|Default|GetGameplayCueTag) (Ability|GameplayCue|MakeGameplayCueParameters :Location _returnvalue_5 :Instigator _returnvalue_3 :EffectCauser _returnvalue_3 :SourceObject _array_element))))))
    (:OnCompleted
      (Ability|EndAbility :!label _label))
    (:OnBlendOut
      (if (Variables|Default|GetEndsOnBlendOut)
        (goto _label)))
    (:OnInterrupted
      (goto _label))
    (:OnCancelled
      (goto _label))))

(fn HandleTargetHit
  (params (TargetedActor :type Actor%20Object%20Reference))
  (bind _output_get (LocalVariables|SetTarget%20Actor TargetedActor))
  (if (Class|AuraAbilitySystemLibrary|AreActorsEnemies (Ability|GetAvatarActorfromActorInfo) _output_get)
    (if (not (GameplayTags|HasMatchingGameplayTag (Ability|GetAbilitySystemComponent (LocalVariables|GetTarget%20Actor)) "(TagName=\"Effects.Invulnerable\")"))
      (Class|AuraDamageGameplayAbility|CauseDamage (LocalVariables|GetTarget%20Actor))
      (Variables|Default|SetTargetWasHit true)
      (bind _returnvalue (Class|CombatInterface|GetHitSound(Message) (LocalVariables|GetTarget%20Actor)))
      (Audio|PlaySoundatLocation _returnvalue (Transformation|GetActorLocation (LocalVariables|GetTarget%20Actor)) "0, 0, 0" 1.0 1.0 0.0 0 0 0 0))))