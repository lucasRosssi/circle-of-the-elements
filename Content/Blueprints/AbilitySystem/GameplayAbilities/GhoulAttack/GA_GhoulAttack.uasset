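; Gameplay Ability for the Ghoul's melee attack, a two-hit right-then-left claw combo.
; On activation it turns the avatar toward its combat target and plays the right montage, chaining into the left one on completion, else ending.
; Each montage waits for an AttackScan gameplay event, then sphere-scans around that hand's socket and damages living enemies in range.
; The ability ends when the second montage finishes or either is interrupted or cancelled.
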(event Ability|EventActivateAbility
  (bind _returnvalue (Ability|GetAvatarActorfromActorInfo))
  (bind _returnvalue_2 (Class|CombatInterface|GetCombatTarget(Message) _returnvalue))
  (Class|CombatInterface|UpdateFacingTarget(Message) _returnvalue (Transformation|GetActorLocation _returnvalue_2))
  (|PlayMontageandWaitProxy "None" "/Game/Assets/Enemies/Ghoul/Animations/AM_Attack_R_Combo_Ghoul.AM_Attack_R_Combo_Ghoul" 1.8 "None" true 1.0 0.0
    (:then
      (Ability|Tasks|WaitGameplayEvent "(TagName=\"Event.Montage.AttackScan\")" 0
        (:EventReceived
          (CallFunction|ScanforTargets "RightHandSocket"))))
    (:OnCompleted
      (|PlayMontageandWaitProxy "None" "/Game/Assets/Enemies/Ghoul/Animations/AM_Attack_L_FromR_Ghoul.AM_Attack_L_FromR_Ghoul" 2.0 "None" true 1.0 0.0
        (:then
          (Ability|Tasks|WaitGameplayEvent "(TagName=\"Event.Montage.AttackScan\")" 0
            (:EventReceived
              (CallFunction|ScanforTargets "LeftHandSocket"))))
        (:OnCompleted
          (Ability|EndAbility :!label _label))
        (:OnInterrupted
          (goto _label))
        (:OnCancelled
          (goto _label))))
    (:OnInterrupted
      (Ability|EndAbility :!label _label_2))
    (:OnCancelled
      (goto _label_2))))

(fn ScanforTargets
  (params (SocketName :type Name))
  (bind _returnvalue (Ability|GetAvatarActorfromActorInfo))
  (bind _returnvalue_2 (Class|CombatInterface|GetAbilitySocketLocation(Message) _returnvalue SocketName false))
  (bind _outoverlappingactors (Class|AuraAbilitySystemLibrary|GetAliveCharactersWithinRadius _returnvalue (Utilities|Array|MakeArray _returnvalue) 4e+01 _returnvalue_2))
  (for _array_element _outoverlappingactors
    (if (Class|AuraAbilitySystemLibrary|AreActorsEnemies (Ability|GetAvatarActorfromActorInfo) _array_element)
      (Class|AuraDamageGameplayAbility|CauseDamage _array_element))))