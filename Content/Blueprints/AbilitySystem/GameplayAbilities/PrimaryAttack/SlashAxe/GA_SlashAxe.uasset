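; Gameplay ability for a slash axe attack that turns the avatar toward the point under the mouse and plays the slash montage.
; Target data from under the mouse sets the facing, then a montage gameplay event marks the strike.
; On that event it only draws a debug sphere at the Vilkar character's weapon socket, with no damage applied here.
; The ability ends when the montage completes, blends out, is interrupted or is cancelled.
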(event Ability|EventActivateAbility
  (bind _datahandle (|TargetDataUnderMouse)
    (:ValidData
      (Variables|Default|SetTargetLocation (.Location (Collision|BreakHitResult (Ability|TargetData|GetHitResultfromTargetData _datahandle))))
      (Class|CombatInterface|UpdateFacingTarget(Message) (Ability|GetAvatarActorfromActorInfo) (Variables|Default|GetTargetLocation))
      (|PlayMontageandWaitProxy "None" "/Game/Assets/Characters/Vilkar/Animations/Abilities/AM_SlashAxe.AM_SlashAxe" 0.8 "None" true 1.0 0.0
        (:then
          (Ability|Tasks|WaitGameplayEvent "(TagName=\"Event.Montage.SlashAxe\")" 0
            (:EventReceived
              (bind _asbp_vilkar_character (Utilities|Casting|CastToBP_VilkarCharacter (Ability|GetAvatarActorfromActorInfo)))
              (Rendering|Debug|DrawDebugSphere (Transformation|GetSocketLocation (Variables|/Script/Aura.AuraCharacterBase|GetWeapon _asbp_vilkar_character) (Variables|/Script/Aura.AuraCharacterBase|GetWeaponProjectileSocketName _asbp_vilkar_character)) 7e+01 8 "(R=0.025275,G=1.000000,B=0.987457,A=1.000000)" 5.0))))
        (:OnCompleted
          (Ability|EndAbility :!label _label))
        (:OnBlendOut
          (goto _label))
        (:OnInterrupted
          (goto _label))
        (:OnCancelled
          (goto _label))))))

(event Ability|EventOnEndAbility
  (params (bWasCancelled :type Boolean)))