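; Primary attack gameplay ability that casts an energy bolt toward an aimed location.
; The target comes from controller input direction on gamepad, with a debug sphere drawn there, or from target data under the mouse otherwise.
; The avatar turns toward the target and plays a cast montage, whose gameplay event spawns the projectile from the weapon's tip socket.
; The ability ends when the montage completes, blends out, or is interrupted or cancelled.
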(event Ability|EventActivateAbility
  (if (Class|AuraGameplayAbility|IsUsingGamepad)
    (bind _output_get (Variables|Default|SetProjectileTargetLocation (+ (* (Variables|/Script/Aura.MainPlayerController|GetInputDirection (Class|AuraGameplayAbility|GetAvatarActorController)) 1e+03) (Transformation|GetActorLocation (Ability|GetAvatarActorfromActorInfo)))))
    (Rendering|Debug|DrawDebugSphere _output_get 1e+02 12 "(R=0.748857,G=0.000000,B=1.000000,A=1.000000)" 2.0 2.0)
    (else
      (bind _datahandle (|TargetDataUnderMouse)
        (:ValidData
          (Variables|Default|SetProjectileTargetLocation (.Location (Collision|BreakHitResult (Ability|TargetData|GetHitResultfromTargetData _datahandle))))))))
  (Class|CombatInterface|UpdateFacingTarget(Message) (Ability|GetAvatarActorfromActorInfo) (Variables|Default|GetProjectileTargetLocation))
  (|PlayMontageandWaitProxy "None" "/Game/Assets/Characters/Aura/Animations/Abilities/AM_Cast_EnergyBolt.AM_Cast_EnergyBolt" 0.8 "None" true 1.0 0.0
    (:then
      (Ability|Tasks|WaitGameplayEvent "(TagName=\"Event.Montage.SpawnProjectile\")" 0
        (:EventReceived
          (Class|ProjectileSpell|SpawnProjectile (Variables|Default|GetProjectileTargetLocation) "TipSocket" true))))
    (:OnCompleted
      (Ability|EndAbility :!label _label))
    (:OnBlendOut
      (goto _label))
    (:OnInterrupted
      (goto _label))
    (:OnCancelled
      (goto _label))))

(event Ability|EventOnEndAbility
  (params (bWasCancelled :type Boolean)))