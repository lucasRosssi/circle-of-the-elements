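; Gameplay ability that makes its avatar play a hit reaction when activated.
; It applies the GE_HitReact effect, plays the avatar-supplied hit react montage at double rate and ends on blend out, interrupt or cancel.
; While it runs, it sets a HitReacting blackboard bool for AI-controlled avatars.
; On end it removes the effect by its stored handle and clears the bool.
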(event Ability|EventActivateAbility
  (bind _returnvalue (Ability|ApplyGameplayEffectToOwner "/Game/Blueprints/AbilitySystem/GameplayEffects/GE_HitReact.GE_HitReact_C"))
  (Variables|Default|SetActive%20GE%20Hit%20React _returnvalue)
  (bind _returnvalue_2 (Class|CombatInterface|GetHitReactMontage(Message) (Ability|GetAvatarActorfromActorInfo)))
  (|PlayMontageandWaitProxy "None" _returnvalue_2 2.0 "None" false 1.0 0.0
    (:then
      (CallFunction|SetBlackboardHitReacting true))
    (:OnBlendOut
      (Ability|EndAbility :!label _label))
    (:OnInterrupted
      (goto _label))
    (:OnCancelled
      (goto _label))))

(event Ability|EventOnEndAbility
  (params (bWasCancelled :type Boolean))
  (Ability|RemoveGameplayEffectFromOwnerWithHandle (Variables|Default|GetActive%20GE%20Hit%20React))
  (CallFunction|SetBlackboardHitReacting false))

(fn SetBlackboardHitReacting
  (params (HitReacting :type Boolean))
  (bind _returnvalue (Ability|GetAvatarActorfromActorInfo))
  (bind _returnvalue_2 (AI|GetAIController _returnvalue))
  (Utilities|IsValid _returnvalue_2
    (:Is%20Valid
      (AI|Components|Blackboard|SetValueasBool (Variables|/Script/AIModule.AIController|GetBlackboard _returnvalue_2) (Variables|Default|GetHitReactingKeyName) HitReacting))))