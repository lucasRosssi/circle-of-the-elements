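; Base gameplay ability that spawns an area effect actor at a targeted world location.
; Player casts show a radius targeting actor and take the impact point from target data on confirm; other casts aim at the combat target's location.
; Both paths face the origin and play a montage, whose SpawnProjectile event spawns the effect and commits the ability on authority.
; Cancelling targeting or finishing the montage ends the ability, hiding the targeting actor.
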(event Ability|EventOnEndAbility
  (params (bWasCancelled :type Boolean))
  (Class|PlayerInterface|HideTargetingActor(Message) (Ability|GetAvatarActorfromActorInfo)))

(event Ability|EventActivateAbility
  (bind _returnvalue (Ability|GetAvatarActorfromActorInfo))
  (bind _returnvalue_2 (Ability|GetAvatarActorfromActorInfo))
  (if (Variables|Default|GetbIsPlayerAbility)
    ;[1 1 1] Targeting State
    (Class|PlayerInterface|ShowTargetingActor(Message) (Ability|GetAvatarActorfromActorInfo) (Variables|Default|GetTargetingActorClass) (Variables|Default|GetAbilityTargetTeam) (Utilities|Struct|BreakScalableFloat (Variables|Default|GetAreaOuterRadius)))
    (|WaitConfirmCancel
      (:OnConfirm
        (bind _datahandle (|TargetData)
          (:ValidData
            (bind _output_get (Variables|Default|SetAreaOrigin (.ImpactPoint (Collision|BreakHitResult (Ability|TargetData|GetHitResultfromTargetData _datahandle)))))
            (Class|CombatInterface|UpdateFacingTarget(Message) _returnvalue _output_get)
            (Class|PlayerInterface|HideTargetingActor(Message) _returnvalue)
            (|PlayMontageandWaitProxy "None" (Variables|Default|GetMontageToPlay) (Class|ActiveAbility|GetMontagePlayRate) "None" true (Class|ActiveAbility|GetAnimRootMotionTranslateScale) 0.0 :!label _label
              (:then
                (Ability|Tasks|WaitGameplayEvent "(TagName=\"Event.Montage.SpawnProjectile\")" 0
                  (:EventReceived
                    (Class|AreaEffectActorAbility|SpawnEffectActor (Variables|Default|GetAreaOrigin))
                    (Ability|HasAuthority
                      (:True
                        (Ability|CommitAbility))))))
              (:OnCompleted
                (Ability|EndAbility :!label _label_2))
              (:OnInterrupted
                (goto _label_2))
              (:OnCancelled
                (goto _label_2))))))
      (:OnCancel
        (Ability|EndAbility)))
    (else
      (bind _returnvalue_3 (Class|CombatInterface|GetCombatTarget(Message) _returnvalue_2))
      (Class|CombatInterface|UpdateFacingTarget(Message) _returnvalue_2 (Transformation|GetActorLocation _returnvalue_3))
      (Variables|Default|SetAreaOrigin (Transformation|GetActorLocation _returnvalue_3))
      (goto _label))))