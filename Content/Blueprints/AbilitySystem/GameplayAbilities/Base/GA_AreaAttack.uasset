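; Base gameplay ability for a targeted area attack that hits living enemies within a radius of a chosen point.
; On activation it shows a targeting actor and waits for confirm or cancel, then takes the confirmed impact point, faces it and plays a montage.
; The montage's SpawnProjectile event fires a burst cue sized by the radius and applies the ability effect in that area.
; Commit happens only after the effects are applied.
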(event Custom|Event%20TargetSet
  ;[0.6106 0.2968 1] Effective State
  (bind _datahandle (|TargetData)
    (:ValidData
      (bind _output_get (Variables|Default|SetAreaOrigin (.ImpactPoint (Collision|BreakHitResult (Ability|TargetData|GetHitResultfromTargetData _datahandle)))))
      (Class|CombatInterface|UpdateFacingTarget(Message) (Ability|GetAvatarActorfromActorInfo) _output_get)
      (|PlayMontageandWaitProxy "None" (Variables|Default|GetMontageToPlay) (Variables|Default|GetMontagePlayRate) "None" true (Variables|Default|GetAnimRootMotionTranslateScale) 0.0
        (:then
          (Ability|Tasks|WaitGameplayEvent "(TagName=\"Event.Montage.SpawnProjectile\")" 0
            (:EventReceived
              (Class|GameplayAbility|ExecuteGameplayCuewithParams (Variables|Default|GetAreaBurstGC) (Ability|GameplayCue|MakeGameplayCueParameters :NormalizedMagnitude (Variables|Default|GetAreaOuterRadius) :Location (Variables|Default|GetAreaOrigin)))
              (CallFunction|ApplyDamagetoArea))))
        (:OnCompleted
          (Ability|EndAbility :!label _label))
        (:OnBlendOut
          (goto _label))
        (:OnInterrupted
          (goto _label))
        (:OnCancelled
          (goto _label))))))

(event Ability|EventActivateAbility
  (EventDispatchers|BindEventtoTargetSet (delegate Custom|Event%20TargetSet))
  ;[1 1 1] Targeting State
  (Class|PlayerInterface|ShowTargetingActor(Message) (Ability|GetAvatarActorfromActorInfo) (Variables|Default|GetTargetingActorClass) "Enemies" (Variables|Default|GetAreaOuterRadius))
  (|WaitConfirmCancel
    (:OnConfirm
      (Default|CallTargetSet))
    (:OnCancel
      (Ability|EndAbility)))
  (Class|PlayerInterface|HideTargetingActor(Message) (Ability|GetAvatarActorfromActorInfo)))

(event Ability|EventOnEndAbility
  (params (bWasCancelled :type Boolean))
  (Class|PlayerInterface|HideTargetingActor(Message) (Ability|GetAvatarActorfromActorInfo)))

(fn ApplyDamagetoArea
  (bind _outoverlappingactors (Class|AuraAbilitySystemLibrary|GetAliveCharactersWithinRadius (Ability|GetAvatarActorfromActorInfo) (Utilities|Array|MakeArray 0) (Variables|Default|GetAreaOuterRadius) (Variables|Default|GetAreaOrigin) "Enemies"))
  (for _array_element _outoverlappingactors
    (Class|AuraAbilitySystemLibrary|ApplyAbilityEffect (Class|BaseAbility|MakeAbilityParamsfromDefaults _array_element)))
  (Ability|CommitAbility)
  (Ability|EndAbility))