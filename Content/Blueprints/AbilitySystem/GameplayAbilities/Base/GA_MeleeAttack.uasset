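; Base melee attack gameplay ability that turns the avatar toward the cursor target (player) or combat target (AI), then plays an attack montage.
; Montage gameplay events either open and close a weapon collision window or trigger a socket-centered radius scan, which also fires a GameplayCue on hit.
; Enemy hits receive the ability effect with the avatar's forward vector.
; Input pressed during the montage chains the next combo montage on blend out.
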(event Custom|OnComponentBeginOverlap_Event
  (params (OverlappedComponent :type Primitive%20Component%20Object%20Reference) (OtherActor :type Actor%20Object%20Reference) (OtherComp :type Primitive%20Component%20Object%20Reference) (OtherBodyIndex :type Integer) (bFromSweep :type Boolean) (SweepResult :type Hit%20Result%20Structure%20%28by%20ref%29))
  ;[1 0.2406 0.2406] Handle Melee Impact
  (CallFunction|OnWeaponCollision OtherActor))

(event Custom|Event%20OnNextComboSequence
  (|PlayMontageandWaitProxy "None" (Class|ActiveDamageAbility|GetAnimMontage) (Class|ActiveAbility|GetMontagePlayRate) "None" true (Class|ActiveAbility|GetAnimRootMotionTranslateScale) 0.0
    (:then
      (Ability|Tasks|WaitInputPress false
        (:then
          ;[1 0.2406 0.2406] Handle Melee Impact
          (if (Variables|Default|GetbWithWeaponCollision)
            (Ability|Tasks|WaitGameplayEvent "(TagName=\"Event.Montage.WeaponCollisionStart\")" 0
              (:EventReceived
                (bind _returnvalue (Class|CombatInterface|EnableWeaponCollision(Message) (Ability|GetAvatarActorfromActorInfo) true))
                (Collision|AssignOnComponentBeginOverlap _returnvalue (delegate Custom|OnComponentBeginOverlap_Event))
                (Ability|Tasks|WaitGameplayEvent "(TagName=\"Event.Montage.WeaponCollisionEnd\")" 0
                  (:EventReceived
                    (CallFunction|StopWeaponCollision)))))
            (else
              (Ability|Tasks|WaitGameplayEvent "(TagName=\"Event.Montage.AttackScan\")" 0
                (:EventReceived
                  (CallFunction|ExecuteAttackScan))))))
        (:OnPress
          (Variables|Default|SetbComboInputPressed true))))
    (:OnCompleted
      (Ability|EndAbility :!label _label))
    (:OnBlendOut
      ;[0.5073 1 0.9343] Handle Combo Sequence
      (if (Variables|Default|GetbComboInputPressed)
        (Math|Integer|IncrementInt (Variables|Default|GetComboIndex)
          (:%20%20
            (Variables|Default|SetbComboInputPressed false)
            (if (Utilities|Array|IsValidIndex (Variables|Default|GetComboSequenceMontages) (Variables|Default|GetComboIndex))
              (Default|CallOnNextComboSequence))))))
    (:OnInterrupted
      (goto _label))
    (:OnCancelled
      (goto _label))))

(event Ability|EventActivateAbility
  (if (Variables|Default|GetbIsComboSequence)
    (EventDispatchers|BindEventtoOnNextComboSequence (delegate Custom|Event%20OnNextComboSequence)))
  (if (Variables|Default|GetbIsPlayerAbility)
    (bind _datahandle (|TargetDataUnderMouse)
      (:ValidData
        (CallFunction|FacetoTarget _datahandle)))
    (else
      (CallFunction|GetAITargetData)))
  (|PlayMontageandWaitProxy "None" (Class|ActiveDamageAbility|GetAnimMontage) (Class|ActiveAbility|GetMontagePlayRate) "None" true (Class|ActiveAbility|GetAnimRootMotionTranslateScale) 0.0
    (:then
      (Ability|Tasks|WaitInputPress false
        (:then
          ;[1 0.2406 0.2406] Handle Melee Impact
          (if (Variables|Default|GetbWithWeaponCollision)
            (Ability|Tasks|WaitGameplayEvent "(TagName=\"Event.Montage.WeaponCollisionStart\")" 0
              (:EventReceived
                (bind _returnvalue (Class|CombatInterface|EnableWeaponCollision(Message) (Ability|GetAvatarActorfromActorInfo) true))
                (Collision|AssignOnComponentBeginOverlap _returnvalue (delegate Custom|OnComponentBeginOverlap_Event))
                (Ability|Tasks|WaitGameplayEvent "(TagName=\"Event.Montage.WeaponCollisionEnd\")" 0
                  (:EventReceived
                    (CallFunction|StopWeaponCollision)))))
            (else
              (Ability|Tasks|WaitGameplayEvent "(TagName=\"Event.Montage.AttackScan\")" 0
                (:EventReceived
                  (CallFunction|ExecuteAttackScan))))))
        (:OnPress
          (Variables|Default|SetbComboInputPressed true))))
    (:OnCompleted
      (Ability|EndAbility :!label _label))
    (:OnBlendOut
      ;[0.5073 1 0.9343] Handle Combo Sequence
      (if (Variables|Default|GetbComboInputPressed)
        (Math|Integer|IncrementInt (Variables|Default|GetComboIndex)
          (:%20%20
            (Variables|Default|SetbComboInputPressed false)
            (if (Utilities|Array|IsValidIndex (Variables|Default|GetComboSequenceMontages) (Variables|Default|GetComboIndex))
              (Default|CallOnNextComboSequence))))))
    (:OnInterrupted
      (goto _label))
    (:OnCancelled
      (goto _label))))

(event Ability|EventOnEndAbility
  (params (bWasCancelled :type Boolean))
  (if (Variables|Default|GetbWithWeaponCollision)
    (CallFunction|StopWeaponCollision)
    (EventDispatchers|UnbindallEventsfromOnNextComboSequence)))

(fn HandleTargetHit
  (params (TargetedActor :type Actor%20Object%20Reference))
  (LocalVariables|SetTarget%20Actor TargetedActor)
  (bind _abilityparams (CallFunction|MakeAbilityParamswithForwardVector (LocalVariables|GetTarget%20Actor)))
  (bind _bsuccess (Class|AuraAbilitySystemLibrary|ApplyAbilityEffect _abilityparams))
  (bind _output_get (Variables|Default|SetTargetWasHit _bsuccess))
  (if _output_get
    _))

(fn MakeAbilityParamswithForwardVector
  (params (TargetActor :type Actor%20Object%20Reference))
  (bind _returnvalue (Class|BaseAbility|MakeAbilityParamsfromDefaults TargetActor))
  (bind (_worldcontextobject _sourceasc _targetasc _abilitylevel _damageparams _effectparams) (Utilities|Struct|BreakAbilityParams _returnvalue))
  (return (Utilities|Struct|MakeAbilityParams _worldcontextobject _sourceasc _targetasc _abilitylevel _damageparams _effectparams (Transformation|GetActorForwardVector (Ability|GetAvatarActorfromActorInfo)))))

(fn GetAITargetData
  (bind _returnvalue (Ability|GetAvatarActorfromActorInfo))
  (Variables|Default|SetTargetWasHit false)
  (bind _returnvalue_2 (Class|CombatInterface|GetCombatTarget(Message) _returnvalue))
  (Class|CombatInterface|UpdateFacingTarget(Message) _returnvalue (Transformation|GetActorLocation _returnvalue_2)))

(fn ExecuteAttackScan
  (bind _returnvalue (Ability|GetAvatarActorfromActorInfo))
  (bind _returnvalue_2 (Ability|GetAvatarActorfromActorInfo))
  (bind _returnvalue_3 (Class|CombatInterface|GetAbilitySocketLocation(Message) (Ability|GetAvatarActorfromActorInfo) (Variables|Default|GetAbilitySocketName) (Variables|Default|GetbUseWeapon)))
  (bind _outoverlappingactors (Class|AuraAbilitySystemLibrary|GetAliveCharactersWithinRadius _returnvalue (Utilities|Array|MakeArray _returnvalue) (Variables|Default|GetMeleeHitScanRadius) _returnvalue_3 "Enemies"))
  (for _array_element _outoverlappingactors
    (CallFunction|HandleTargetHit _array_element))
  (if (Variables|Default|GetTargetWasHit)
    (Class|GameplayAbility|ExecuteGameplayCuewithParams (Variables|Default|GetGameplayCueTag) (Ability|GameplayCue|MakeGameplayCueParameters :Location _returnvalue_3 :Instigator _returnvalue_2 :EffectCauser _returnvalue_2 :SourceObject _array_element))))

(fn OnWeaponCollision
  (params (HitActor :type Actor%20Object%20Reference))
  (if (Class|AuraAbilitySystemLibrary|AreActorsEnemies (Ability|GetAvatarActorfromActorInfo) HitActor)
    (CallFunction|HandleTargetHit HitActor)))

(fn StopWeaponCollision
  (bind _returnvalue (Class|CombatInterface|EnableWeaponCollision(Message) (Ability|GetAvatarActorfromActorInfo) false))
  (EventDispatchers|UnbindallEventsfromOnComponentBeginOverlap _returnvalue))

(fn FacetoTarget
  (params (HitResult :type Gameplay%20Ability%20Target%20Data%20Handle%20Structure%20%28by%20ref%29))
  (Class|CombatInterface|UpdateFacingTarget(Message) (Ability|GetAvatarActorfromActorInfo) (.Location (Collision|BreakHitResult (Ability|TargetData|GetHitResultfromTargetData HitResult)))))