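; Base gameplay ability for a montage-driven projectile attack, shared by player and non-player characters.
; Player abilities face the mouse target data hit point, while others face their combat target and store its location as the projectile target.
; A montage gameplay event spawns the projectile from the configured socket toward TargetLocation, then commits the ability.
; The ability ends when the montage completes, is interrupted or is cancelled.
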(event Ability|EventActivateAbility
  (bind _returnvalue (Ability|GetAvatarActorfromActorInfo))
  (if (Variables|Default|GetPlayerAbility)
    (bind _datahandle (|TargetDataUnderMouse)
      (:ValidData
        (Class|CombatInterface|UpdateFacingTarget(Message) (Ability|GetAvatarActorfromActorInfo) (.Location (Collision|BreakHitResult (Ability|TargetData|GetHitResultfromTargetData _datahandle))))))
    (else
      (bind _returnvalue_2 (Class|CombatInterface|GetCombatTarget(Message) _returnvalue))
      (Class|CombatInterface|UpdateFacingTarget(Message) _returnvalue (Transformation|GetActorLocation _returnvalue_2))
      (Variables|Default|SetTargetLocation (Transformation|GetActorLocation _returnvalue_2))))
  (|PlayMontageandWaitProxy "None" (Variables|Default|GetAbilityMontage) 1.0 "None" true 1.0 0.0
    (:then
      (Ability|Tasks|WaitGameplayEvent "(TagName=\"Event.Montage.SpawnProjectile\")" 0
        (:EventReceived
          (Class|ProjectileSpell|SpawnProjectile (Variables|Default|GetTargetLocation) (Variables|Default|GetProjectileSpawnSocketName) (Variables|Default|GetSocket%20in%20Weapon))
          (Ability|CommitAbility))))
    (:OnCompleted
      (Ability|EndAbility :!label _label))
    (:OnInterrupted
      (goto _label))
    (:OnCancelled
      (goto _label))))