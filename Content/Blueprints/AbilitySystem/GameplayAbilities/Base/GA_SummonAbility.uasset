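; Base summon gameplay ability that spawns minions at shuffled locations, ending immediately if the maximum is already active.
; It plays a montage, waits for the Summon gameplay event, then loops through locations with short random delays, spawning a Niagara effect and minion at each.
; Each minion's destroyed event decrements the active count.
; The ability ends after the last spawn or on montage interruption or cancellation, resetting the location index.
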(event Custom|On%20Minion%20Destroyed
  (params (DestroyedActor :type Actor%20Object%20Reference))
  (Math|Integer|DecrementInt (Variables|Default|GetActiveMinions)))

(event Ability|EventActivateAbility
  (if (Class|SummonAbility|HasMaxMinionsActive)
    (Ability|EndAbility)
    (else
      (bind _returnvalue (Class|SummonAbility|GetSpawnLocations))
      (bind _output_get (Variables|Default|SetSpawnLocations _returnvalue))
      (Utilities|Array|Shuffle _output_get)
      (|PlayMontageandWaitProxy "None" (Variables|Default|GetMontageToPlay) (Class|ActiveAbility|GetMontagePlayRate) "None" true (Class|ActiveAbility|GetAnimRootMotionTranslateScale) 0.0
        (:then
          (Ability|Tasks|WaitGameplayEvent "(TagName=\"Event.Montage.Summon\")" 0
            (:EventReceived
              (if (< (Variables|Default|GetSpawnLocationIndex) (Utilities|Array|Length (Variables|Default|GetSpawnLocations))) :!label _label
                (Niagara|SpawnSystematLocation "/Game/Assets/Effects/Summon/NS_SummonSpawnArea.NS_SummonSpawnArea" (Utilities|Array|Get(acopy) (Variables|Default|GetSpawnLocations) (Variables|Default|GetSpawnLocationIndex)))
                (bind _returnvalue_2 (Class|SummonAbility|SpawnMinion (Utilities|Array|Get(acopy) (Variables|Default|GetSpawnLocations) (Variables|Default|GetSpawnLocationIndex))))
                (Utilities|IsValid _returnvalue_2
                  (:Is%20Valid
                    (Game|BindEventtoOnDestroyed _returnvalue_2 (delegate Custom|On%20Minion%20Destroyed)))
                  (:Is%20Not%20Valid
                    _))
                (Math|Integer|IncrementInt (Variables|Default|GetSpawnLocationIndex)
                  (:%20%20
                    (Utilities|FlowControl|Delay (Math|Random|RandomFloatinRange 0.0 0.3))
                    (goto _label)))
                (else
                  (Ability|EndAbility))))))
        (:OnInterrupted
          (Ability|EndAbility :!label _label_2))
        (:OnCancelled
          (goto _label_2))))))

(event Ability|EventOnEndAbility
  (params (bWasCancelled :type Boolean))
  (Variables|Default|SetSpawnLocationIndex 0))