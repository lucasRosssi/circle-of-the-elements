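; Gameplay ability that summons randomly chosen minions around a set of computed spawn locations, each with a ground summon Niagara effect.
; On activation it stores and shuffles the locations, then spawns each minion facing the avatar's direction.
; A hand-built loop with short random delays staggers the spawns and ends the ability after the last location.
; The loop index is never reset in this graph.
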(event Ability|EventActivateAbility
  (bind _returnvalue (Class|SummonAbility|GetSpawnLocations))
  (bind _output_get (Variables|Default|SetSpawnLocations _returnvalue))
  (Utilities|Array|Shuffle _output_get)
  (if (< (Variables|Default|GetSpawnLocationIndex) (Utilities|Array|Length (Variables|Default|GetSpawnLocations))) :!label _label
    (Niagara|SpawnSystematLocation "/Game/Assets/Effects/Combat/NS_GroundSummon.NS_GroundSummon" (Utilities|Array|Get(acopy) (Variables|Default|GetSpawnLocations) (Variables|Default|GetSpawnLocationIndex)))
    (Class|SummonAbility|SpawnMinion (Class|SummonAbility|GetRandomMinionClass) (Utilities|Array|Get(acopy) (Variables|Default|GetSpawnLocations) (Variables|Default|GetSpawnLocationIndex)) (Transformation|GetActorRotation (Ability|GetAvatarActorfromActorInfo)))
    (Math|Integer|IncrementInt (Variables|Default|GetSpawnLocationIndex)
      (:%20%20
        (Utilities|FlowControl|Delay (Math|Random|RandomFloatinRange 0.0 0.3))
        (goto _label)))
    (else
      (Ability|EndAbility))))

(event Ability|EventOnEndAbility
  (params (bWasCancelled :type Boolean)))