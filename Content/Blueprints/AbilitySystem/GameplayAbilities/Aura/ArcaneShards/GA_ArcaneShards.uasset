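; GA_ArcaneShards is the Arcane Shards gameplay ability, currently implementing only its targeting phase with debug prints and no damage or spawning.
; On activation it starts a Targeting ability state and tells the avatar, via interface message, to show a targeting actor.
; An input press hides that actor and ends the state.
; The state-ended branch then waits for input release to end the ability.
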(event Ability|EventActivateAbility
  (|StartAbilityState (Variables|Default|GetTargeting) true
    (:then
      (Development|PrintString "Targeting Start!")
      (Class|PlayerInterface|ShowTargetingActor(Message) (Ability|GetAvatarActorfromActorInfo) (Variables|Default|GetTargetingActorClass))
      (Ability|Tasks|WaitInputPress false
        (:OnPress
          (Class|PlayerInterface|HideTargetingActor(Message) (Ability|GetAvatarActorfromActorInfo))
          (Class|GameplayAbility|EndAbilityState (Variables|Default|GetTargeting)))))
    (:OnStateEnded
      (Development|PrintString "Targeting Ended!")
      (Ability|Tasks|WaitInputRelease false
        (:OnRelease
          (Ability|EndAbility))))))