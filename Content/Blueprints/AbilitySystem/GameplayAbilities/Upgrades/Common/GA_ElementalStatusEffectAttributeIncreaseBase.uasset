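; Base upgrade ability that rewards applying elemental status effects with attribute increases and essence.
; On activation it listens for gameplay effects applied to targets that match a tag requirement and counts them.
; When the count reaches a level-scaled threshold, it resets and sends a message adding one to the configured attribute on the avatar.
; Each application also rolls a level-scaled chance to send a message granting one essence resource.
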(event Ability|EventActivateAbility
  (Ability|Tasks|WaitGameplayEffectAppliedToTarget :TargetTagRequirements (Variables|Default|GetEffectTargetTagRequirements) :OptionalExternalOwner 0
    (:OnApplied
      (bind _result (Math|Integer|IncrementInt (Variables|Default|GetEffectCount))
        (:%20%20
          (Development|PrintString (Utilities|String|ToString(Integer) _result))
          (CallFunction|CheckApplyCountandIncreaseAttribute)
          (if (CallFunction|RollEssenceChance)
            (Class|PlayerInterface|AddResource(Message) (Ability|GetAvatarActorfromActorInfo) (Variables|Default|GetEssenceTag) 1)))))))

(fn RollEssenceChance
  (return (<= (Math|Random|RandomFloatinRange 0.0 1.0) (Class|UtilityLibrary|GetScalableFloatatLevel (Variables|Default|GetEssenceChance) (Ability|GetAbilityLevel)))))

(fn CheckApplyCountandIncreaseAttribute
  (if (>= (Variables|Default|GetEffectCount) (Class|UtilityLibrary|GetScalableIntegeratLevel (Variables|Default|GetEffectThreshold) (Ability|GetAbilityLevel)))
    (Variables|Default|SetEffectCount 0)
    (Class|PlayerInterface|AddAttribute(Message) (Ability|GetAvatarActorfromActorInfo) (Variables|Default|GetAttributeTag) 1)))