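; Pyromania fire upgrade ability that rewards the avatar for applying tag-filtered effects, counted as burns, with Intelligence and essence.
; It listens for gameplay effects the owner applies to targets, including periodic ones, and increments a burn counter each time.
; Reaching the threshold resets the counter and adds an Intelligence point, while every application also rolls for one essence.
; Threshold and essence chance scale with ability level.
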(event Ability|EventActivateAbility
  (Ability|Tasks|WaitGameplayEffectAppliedToTarget :TargetTagRequirements (Variables|Default|GetTarget%20Tag%20Requirements) :OptionalExternalOwner 0 :ListenForPeriodicEffects true
    (:OnApplied
      (Math|Integer|IncrementInt (Variables|Default|GetBurnCount)
        (:%20%20
          (CallFunction|CheckBurnCountandIncreaseIntelligence)
          (if (CallFunction|RollEssenceChance)
            (Class|PlayerInterface|AddResource(Message) (Ability|GetAvatarActorfromActorInfo) (Variables|Default|GetEssenceTag) 1)))))))

(fn RollEssenceChance
  (return (<= (Math|Random|RandomFloatinRange 0.0 1.0) (Class|UtilityLibrary|GetScalableFloatatLevel (Variables|Default|GetEssenceChance) (Ability|GetAbilityLevel)))))

(fn CheckBurnCountandIncreaseIntelligence
  (if (>= (Variables|Default|GetBurnCount) (Class|UtilityLibrary|GetScalableIntegeratLevel (Variables|Default|GetBurnThreshold) (Ability|GetAbilityLevel)))
    (Variables|Default|SetBurnCount 0)
    (Class|PlayerInterface|AddAttribute(Message) (Ability|GetAvatarActorfromActorInfo) (Variables|Default|GetIntelligenceTag) 1)))