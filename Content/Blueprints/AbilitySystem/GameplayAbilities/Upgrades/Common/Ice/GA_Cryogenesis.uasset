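; GA_Cryogenesis is an Ice upgrade gameplay ability that rewards its owner for applying chill effects to targets.
; It waits for tag-filtered gameplay effects applied to targets and counts each one, printing the count.
; When the count reaches a level-scaled threshold, it resets and adds one Wisdom to the avatar.
; Each application also rolls a level-scaled chance to grant one Essence resource.
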(event Ability|EventActivateAbility
  (Ability|Tasks|WaitGameplayEffectAppliedToTarget :TargetTagRequirements (Variables|Default|GetTarget%20Tag%20Requirements) :OptionalExternalOwner 0
    (:OnApplied
      (bind _result (Math|Integer|IncrementInt (Variables|Default|GetChillCount))
        (:%20%20
          (Development|PrintString (Utilities|String|ToString(Integer) _result))
          (CallFunction|CheckChillCountandIncreaseWisdom)
          (if (CallFunction|RollEssenceChance)
            (Class|PlayerInterface|AddResource(Message) (Ability|GetAvatarActorfromActorInfo) (Variables|Default|GetEssenceTag) 1)))))))

(fn RollEssenceChance
  (return (<= (Math|Random|RandomFloatinRange 0.0 1.0) (Class|UtilityLibrary|GetScalableFloatatLevel (Variables|Default|GetEssenceChance) (Ability|GetAbilityLevel)))))

(fn CheckChillCountandIncreaseWisdom
  (if (>= (Variables|Default|GetChillCount) (Class|UtilityLibrary|GetScalableIntegeratLevel (Variables|Default|GetChillThreshold) (Ability|GetAbilityLevel)))
    (Variables|Default|SetChillCount 0)
    (Class|PlayerInterface|AddAttribute(Message) (Ability|GetAvatarActorfromActorInfo) (Variables|Default|GetWisdomTag) 1)))