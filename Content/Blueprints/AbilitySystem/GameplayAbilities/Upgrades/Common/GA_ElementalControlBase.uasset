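; Base upgrade gameplay ability that grants a random extra attribute amount in response to an elemental gameplay event.
; On activation it waits for ElementTag events, then sends an attribute message for AttributeTag to the avatar actor.
; The amount is a random integer from zero up to the ExtraAttribute scalable value at the current ability level.
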(event Ability|EventActivateAbility
  (Ability|Tasks|WaitGameplayEvent (Variables|Default|GetElementTag) 0
    (:EventReceived
      (Class|PlayerInterface|AddAttribute(Message) (Ability|GetAvatarActorfromActorInfo) (Variables|Default|GetAttributeTag) (CallFunction|RollExtraAttribute)))))

(fn RollExtraAttribute
  (return (Math|Random|RandomIntegerinRange 0 (Class|UtilityLibrary|GetScalableIntegeratLevel (Variables|Default|GetExtraAttribute) (Ability|GetAbilityLevel)))))