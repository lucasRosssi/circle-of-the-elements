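; GA_SoulAbsorption is a Soul upgrade gameplay ability that gives a chance of bonus attribute points from soul essence interactions.
; While active, it waits repeatedly for abilities tagged Abilities.Interaction.SoulEssence to activate and rolls against a level-scaled chance each time.
; On success, it sends the avatar an attribute-points message with a random amount between one and a level-scaled maximum.
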(event Ability|EventActivateAbility
  (|WaitforAbilityActivate :WithTag "(TagName=\"Abilities.Interaction.SoulEssence\")" :TriggerOnce false
    (:OnActivate
      (if (CallFunction|RollExtraAPChance)
        (Class|PlayerInterface|AddAttributePoints(Message) (Ability|GetAvatarActorfromActorInfo) (CallFunction|RollExtraAPAmount))))))

(fn RollExtraAPChance
  (return (<= (Math|Random|RandomFloatinRange 0.0 1.0) (Class|UtilityLibrary|GetScalableFloatatLevel (Variables|Default|GetExtraAPChance) (Ability|GetAbilityLevel)))))

(fn RollExtraAPAmount
  (return (Math|Random|RandomIntegerinRange 1 (Class|UtilityLibrary|GetScalableIntegeratLevel (Variables|Default|GetExtraAP) (Ability|GetAbilityLevel)))))