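; GA_ShortRest is a Soul upgrade gameplay ability that heals its owner up to a health threshold whenever combat finishes.
; On activation it binds to the combat manager's combat-finished delegate, then compares the avatar's health fraction to a threshold scaled by ability level.
; If health is below it, it applies GE_Heal to the owner with a set-by-caller Heal magnitude equal to the missing amount.
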(event Custom|OnCombatFinished
  (params (AreaName :type Name))
  (if (CallFunction|IsHealthLessThenThreshold)
    (CallFunction|HealtoThreshold)))

(event Ability|EventActivateAbility
  (bind _returnvalue (Class|AuraSystemsLibrary|GetCombatManager))
  (Utilities|IsValid _returnvalue
    (:Is%20Valid
      (EventDispatchers|BindEventtoOnCombatFinishedDelegate _returnvalue (EventDispatchers|CreateEvent :!event Custom|OnCombatFinished)))))

(fn IsHealthLessThenThreshold
  (bind _returnvalue (Ability|GetAvatarActorfromActorInfo))
  (bind _returnvalue_2 (Ability|Attribute|GetFloatAttribute _returnvalue "(AttributeName=\"Health\",Attribute=/Script/Aura.AuraAttributeSet:Health,AttributeOwner=/Script/CoreUObject.Class'\"/Script/Aura.AuraAttributeSet\"')"))
  (Variables|Default|SetHealth _returnvalue_2)
  (bind _output_get (Variables|Default|SetMaxHealth (.ReturnValue (Ability|Attribute|GetFloatAttribute (Ability|GetAvatarActorfromActorInfo) "(AttributeName=\"MaxHealth\",Attribute=/Script/Aura.AuraAttributeSet:MaxHealth,AttributeOwner=/Script/CoreUObject.Class'\"/Script/Aura.AuraAttributeSet\"')"))))
  (return (< (/ _returnvalue_2 _output_get) (CallFunction|GetCurrentHealthThreshold))))

(fn GetCurrentHealthThreshold
  (return (Class|UtilityLibrary|GetScalableFloatatLevel (Variables|Default|GetHealthThreshold) (Ability|GetAbilityLevel))))

(fn GetHealingtoThreshold
  (return (- (* (CallFunction|GetCurrentHealthThreshold) (Variables|Default|GetMaxHealth)) (Variables|Default|GetHealth))))

(fn HealtoThreshold
  (bind _returnvalue (Ability|GameplayEffect|AssignTagSetbyCallerMagnitude (Ability|MakeOutgoingGameplayEffectSpec "/Game/Blueprints/AbilitySystem/GameplayEffects/GE_Heal.GE_Heal_C") "(TagName=\"Heal\")" (CallFunction|GetHealingtoThreshold)))
  (Ability|ApplyGameplayEffectSpecToOwner _returnvalue))