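; GA_WildSoul is the gameplay ability for the Wild Soul upgrade, reacting to soul essence interaction events.
; Each event grants the avatar a random number of attribute points, capped by level-scaled ExtraAP, then spends points randomly.
; It then removes effects granting the Upgrades.Soul.Wild tag and reapplies UE_WildSoul only if a level-scaled ExtraEssenceChance roll succeeds.
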(event Ability|EventActivateAbility
  (Ability|Tasks|WaitGameplayEvent "(TagName=\"Abilities.Interaction.SoulEssence\")" 0
    (:EventReceived
      (Class|PlayerInterface|AddAttributePoints(Message) (Ability|GetAvatarActorfromActorInfo) (CallFunction|RollExtraAP))
      (Class|PlayerInterface|SpendAttributePointsRandomly(Message) (Ability|GetAvatarActorfromActorInfo))
      (Ability|RemoveGameplayEffectFromOwnerWithGrantedTags "(GameplayTags=((TagName=\"Upgrades.Soul.Wild\")))")
      (if (CallFunction|RollExtraEssenceChance)
        (Ability|ApplyGameplayEffectToOwner "/Game/Blueprints/AbilitySystem/GameplayEffects/Upgrades/Common/Soul/UE_WildSoul.UE_WildSoul_C" (Ability|GetAbilityLevel))))))

(fn RollExtraAP
  (return (Math|Random|RandomIntegerinRange 1 (Class|UtilityLibrary|GetScalableIntegeratLevel (Variables|Default|GetExtraAP) (Ability|GetAbilityLevel)))))

(fn RollExtraEssenceChance
  (return (<= (Math|Random|RandomFloatinRange 0.0 1.0) (Class|UtilityLibrary|GetScalableFloatatLevel (Variables|Default|GetExtraEssenceChance) (Ability|GetAbilityLevel)))))