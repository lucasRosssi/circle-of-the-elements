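; GA_Respite is a Soul upgrade gameplay ability that gives a level-scaled chance of extra healing when an encounter's last enemy is killed.
; On activation it applies the UE_Respite effect to the owner at the ability level and binds to the encounter manager's last-enemy-killed delegate.
; That event rolls against DoubleHealingChance and, on success, only calls CommitAbility, with no explicit heal in the graph.
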(event Custom|OnLastEnemyKilled
  (if (CallFunction|RollExtraHeal)
    (Ability|CommitAbility)))

(event Ability|EventActivateAbility
  (EventDispatchers|BindEventtoOnLastEnemyKilledDelegate (Class|AuraSystemsLibrary|GetEncounterManager) (EventDispatchers|CreateEvent :!event Custom|OnLastEnemyKilled))
  (Ability|ApplyGameplayEffectToOwner "/Game/Blueprints/AbilitySystem/GameplayEffects/Upgrades/Common/Soul/UE_Respite.UE_Respite_C" (Ability|GetAbilityLevel)))

(fn RollExtraHeal
  (return (<= (Math|Random|RandomFloatinRange 0.0 1.0) (Class|UtilityLibrary|GetScalableFloatatLevel (Variables|Default|GetDoubleHealingChance) (Ability|GetAbilityLevel)))))