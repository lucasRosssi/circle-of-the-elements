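; Second Wind upgrade ability that heals the avatar during an invulnerable, slow-motion cinematic moment.
; Activation applies GE_Dodge, switches the camera state and slows global time, raising custom dilation on the avatar and Niagara effect to partly offset it.
; An intro montage plays with sound and VFX, then a level-scaled, attribute-based heal lands as it blends into the outro.
; Ending the ability removes the invulnerability and restores time and camera.
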(event Ability|EventOnEndAbility
  (params (bWasCancelled :type Boolean))
  (Ability|RemoveGameplayEffectFromOwnerWithHandle (Variables|Default|GetInvulnerableHandle))
  (CallFunction|EndCoolEffects))

(event Ability|EventActivateAbilityFromEvent
  (params (EventData :type Gameplay%20Event%20Data%20Structure%20%28by%20ref%29))
  (bind _returnvalue (Ability|ApplyGameplayEffectToOwner "/Game/Blueprints/AbilitySystem/GameplayEffects/Actions/GE_Dodge.GE_Dodge_C"))
  (Variables|Default|SetInvulnerableHandle _returnvalue)
  (CallFunction|SetCoolEffects)
  (Utilities|WaitMontagesandEffects
    (:OnCompleted
      (Ability|EndAbility))))

(fn ApplyHealing
  (bind _returnvalue (Ability|GetAbilitySystemComponentfromActorInfo))
  (Class|AuraAbilitySystemLibrary|ApplyAbilityEffect (Utilities|Struct|MakeAbilityParams (Ability|GetAvatarActorfromActorInfo) _returnvalue _returnvalue 1 (Utilities|Struct|MakeHealParams "/Game/Blueprints/AbilitySystem/GameplayEffects/GE_Heal.GE_Heal_C" (* (.ReturnValue (Ability|Attribute|GetFloatAttribute (Ability|GetAvatarActorfromActorInfo) "(AttributeName=\"MaxHealth\",Attribute=/Script/Aura.AuraAttributeSet:MaxHealth,AttributeOwner=/Script/CoreUObject.Class'\"/Script/Aura.AuraAttributeSet\"')")) (Class|BaseAbility|GetHealatLevel (Ability|GetAbilityLevel)))))))

(fn SetCoolEffects
  (Class|AuraCamera|SetCameraState (Class|BaseAbility|GetPlayerCamera) "SecondWind")
  (Utilities|Time|SetGlobalTimeDilation 0.1)
  (Variables|/Script/Engine.Actor|SetCustomTimeDilation (Ability|GetAvatarActorfromActorInfo) 5.0))

(fn SpawnSoundandNiagara
  (bind _returnvalue (Class|BaseAbility|GetAvatarCharacter))
  (bind _returnvalue_2 (Transformation|GetActorLocation _returnvalue))
  (Audio|PlaySoundatLocation "/Game/Assets/Sounds/Abilities/FireNado/SFX_Fire-Nado_03.SFX_Fire-Nado_03" (Transformation|GetActorLocation (Ability|GetAvatarActorfromActorInfo)) "0, 0, 0" 0.8 0.7 0.0 0 0 0 0)
  (bind _returnvalue_3 (Niagara|SpawnSystematLocation "/Game/Assets/Effects/Abilities/SecondWind/NS_SecondWind.NS_SecondWind" (Math|Vector|MakeVector (.x _returnvalue_2) (.y _returnvalue_2) (+ (+ (.z _returnvalue_2) (* (Components|Capsule|GetScaledCapsuleHalfHeight (Variables|/Script/Engine.Character|GetCapsuleComponent _returnvalue)) -1.0)) 2.0)) "0, 0, 0" "1.200000,1.200000,1.200000"))
  (bind _output_get (Variables|Default|SetSpawnedNiagara _returnvalue_3))
  (Class|NiagaraComponent|SetCustomTimeDilation _output_get 5.0)
  (return))

(fn EndCoolEffects
  (bind _spawnedniagara (Variables|Default|GetSpawnedNiagara))
  (Utilities|Time|SetGlobalTimeDilation 1.0)
  (Variables|/Script/Engine.Actor|SetCustomTimeDilation (Ability|GetAvatarActorfromActorInfo) 1.0)
  (Utilities|IsValid _spawnedniagara
    (:Is%20Valid
      (Class|NiagaraComponent|SetCustomTimeDilation _spawnedniagara 1.0))
    (:Is%20Not%20Valid
      _))
  (Class|AuraCamera|SetCameraState (Class|BaseAbility|GetPlayerCamera) "Default"))