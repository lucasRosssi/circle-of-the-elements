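; Goblin spear melee ability that turns the enemy toward its combat target and plays the attack montage, ending when the montage completes or is interrupted.
; Montage AttackScan events trigger a small sphere check at the weapon's tip socket, damaging living enemies not tagged invulnerable.
; Hits play each target's hit sound, then one swipe sound and a blood effect from the last scanned character, which may differ from the one hit.
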(event Ability|EventActivateAbility
  (bind _returnvalue (Ability|GetAvatarActorfromActorInfo))
  (bind _returnvalue_2 (Ability|GetAvatarActorfromActorInfo))
  (Variables|Default|SetTargetWasHit false)
  (bind _returnvalue_3 (Class|CombatInterface|GetCombatTarget(Message) _returnvalue))
  (Class|CombatInterface|UpdateFacingTarget(Message) _returnvalue (Transformation|GetActorLocation _returnvalue_3))
  (|PlayMontageandWaitProxy "None" "/Game/Assets/Enemies/Goblin/Animations/Spear/AM_Attack_Spear.AM_Attack_Spear" 1.0 "None" true 1.0 0.0
    (:then
      (Ability|Tasks|WaitGameplayEvent "(TagName=\"Event.Montage.AttackScan\")" 0
        (:EventReceived
          (bind _returnvalue_4 (Class|CombatInterface|GetAbilitySocketLocation(Message) _returnvalue_2 "TipSocket" true))
          (bind _outoverlappingactors (Class|AuraAbilitySystemLibrary|GetAliveCharactersWithinRadius _returnvalue_2 (Utilities|Array|MakeArray _returnvalue_2) 2e+01 _returnvalue_4))
          (for _array_element _outoverlappingactors
            (CallFunction|HandleTargetHit _array_element))
          (if (Variables|Default|GetTargetWasHit)
            (Audio|PlaySoundatLocation "/Game/Assets/Sounds/Enemies/Ghoul/Swipe/sfx_Swipe.sfx_Swipe" _returnvalue_4 "0, 0, 0" 0.75 1.2 0.0 0 0 0 0)
            (bind _returnvalue_5 (Class|CombatInterface|GetBloodEffect(Message) _array_element))
            (Niagara|SpawnSystematLocation _returnvalue_5 _returnvalue_4)))))
    (:OnCompleted
      (Ability|EndAbility :!label _label))
    (:OnInterrupted
      (goto _label))
    (:OnCancelled
      (goto _label))))

(fn HandleTargetHit
  (params (TargetedActor :type Actor%20Object%20Reference))
  (bind _output_get (LocalVariables|SetTarget%20Actor TargetedActor))
  (if (Class|AuraAbilitySystemLibrary|AreActorsEnemies (Ability|GetAvatarActorfromActorInfo) _output_get)
    (if (not (GameplayTags|HasMatchingGameplayTag (Ability|GetAbilitySystemComponent (LocalVariables|GetTarget%20Actor)) "(TagName=\"Effects.Invulnerable\")"))
      (Class|AuraDamageGameplayAbility|CauseDamage (LocalVariables|GetTarget%20Actor))
      (Variables|Default|SetTargetWasHit true)
      (bind _returnvalue (Class|CombatInterface|GetHitSound(Message) (LocalVariables|GetTarget%20Actor)))
      (Audio|PlaySoundatLocation _returnvalue (Transformation|GetActorLocation (LocalVariables|GetTarget%20Actor)) "0, 0, 0" 1.0 1.0 0.0 0 0 0 0))))