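; Crystal Shaman enemy ability that hijacks a random available equipped spirit from its combat target.
; It marks itself as the spirit's hijacker, faces the target and plays a montage while awaiting the Event.Spirit.Hijacked gameplay event.
; On that event it gains the spirit's element tag and hijack-success loose tags; montage interruption or cancellation releases the spirit.
; CommitAbility runs in OnEndAbility, so even failed attempts commit.
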(event Ability|EventActivateAbility
  (bind (_montage _playrate _rootmotionscale) (Class|ActiveAbility|GetMontageParams))
  (bind _returnvalue (Class|CombatInterface|GetCombatTarget(Message) (Ability|GetAvatarActorfromActorInfo)))
  (Variables|Default|SetCombatTarget _returnvalue)
  (bind _returnvalue_2 (Class|CombatInterface|GetAvailableEquippedSpirits(Message) (Variables|Default|GetCombatTarget)))
  (bind _output_get (Variables|Default|SetTargetEquippedSpirits _returnvalue_2))
  (if (Utilities|Array|IsEmpty _output_get)
    (Ability|EndAbility)
    (else
      (bind _output_get_2 (Variables|Default|SetSpiritActor (Class|Spirit|GetSpiritActor (.OutItem (Utilities|Array|Random (Variables|Default|GetTargetEquippedSpirits))))))
      (Class|SpiritActor|SetHijacker _output_get_2 (Ability|GetAvatarActorfromActorInfo))
      (Class|CombatInterface|UpdateFacingTarget(Message) (Ability|GetAvatarActorfromActorInfo) (Transformation|GetActorLocation (Variables|Default|GetCombatTarget)))
      (|PlayMontageandWaitProxy "None" _montage _playrate "None" true _rootmotionscale 0.0 false
        (:then
          (Ability|Tasks|WaitGameplayEvent "(TagName=\"Event.Spirit.Hijacked\")" 0
            (:EventReceived
              (CallFunction|CompleteHijack))))
        (:OnInterrupted
          (Class|SpiritActor|SetHijacker (Variables|Default|GetSpiritActor) :!label _label)
          (Variables|Default|SetSpiritActor 0)
          (Ability|EndAbility))
        (:OnCancelled
          (goto _label))))))

(event Ability|EventOnEndAbility
  (params (bWasCancelled :type Boolean))
  (Ability|CommitAbility))

(fn CompleteHijack
  (GameplayTags|AddGameplayTag (Variables|Default|GetElementTagContainer) (Class|SpiritActor|GetElementTag (Variables|Default|GetSpiritActor)) :!class /Script/GameplayTags.BlueprintGameplayTagLibrary)
  (Ability|GameplayEffect|AddLooseGameplayTags (Ability|GetAvatarActorfromActorInfo) (Variables|Default|GetElementTagContainer))
  (Ability|GameplayEffect|AddLooseGameplayTags (Ability|GetAvatarActorfromActorInfo) (Variables|Default|GetHijackSuccessfulTagContainer))
  (Ability|EndAbility))