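; Volcanic Blast actor for the Blazing Brain enemy ability, playing a timed fiery impact at its location.
; On BeginPlay it waits until shortly before DelayImpact, spawns the impact Niagara system, deactivates its own effect and fades its audio out.
; Layered impact sounds follow a moment later.
; Sphere begin and end overlaps are forwarded to OnOverlap and OnEndOverlap, whose logic is not defined in this graph.
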(event OnComponentBeginOverlap(Sphere)
  (params (OverlappedComponent :type Primitive%20Component%20Object%20Reference) (OtherActor :type Actor%20Object%20Reference) (OtherComp :type Primitive%20Component%20Object%20Reference) (OtherBodyIndex :type Integer) (bFromSweep :type Boolean) (SweepResult :type Hit%20Result%20Structure%20%28by%20ref%29))
  (Class|AreaEffectActor|OnOverlap OtherActor))

(event OnComponentEndOverlap(Sphere)
  (params (OverlappedComponent :type Primitive%20Component%20Object%20Reference) (OtherActor :type Actor%20Object%20Reference) (OtherComp :type Primitive%20Component%20Object%20Reference) (OtherBodyIndex :type Integer))
  (Class|AreaEffectActor|OnEndOverlap OtherActor))

(event EventBeginPlay
  (Utilities|FlowControl|Delay (- (Variables|Default|GetDelayImpact) 0.4))
  (Niagara|SpawnSystematLocation "/Game/Assets/Effects/Abilities/VolcanicBlast/NS_VolcanicBlast_Impact.NS_VolcanicBlast_Impact" (Transformation|GetActorLocation))
  (Components|Activation|Deactivate (Variables|Default|GetNiagara))
  (Audio|Components|Audio|AdjustVolume (Variables|Default|GetAudio) 1.0 0.0 "Linear" :!class /Script/Engine.AudioComponent)
  (Utilities|FlowControl|Delay 0.1)
  (Audio|PlaySoundatLocation "/Game/Assets/Sounds/Abilities/FireBolt/sfx_FireBolt_Impact.sfx_FireBolt_Impact" (Transformation|GetActorLocation) "0, 0, 0" 1.5 0.9 0.0 0 0 0 0)
  (Audio|PlaySoundatLocation "/Game/Assets/Sounds/Elements/Fire/sfx_Fire_Hit_2.sfx_Fire_Hit_2" (Transformation|GetActorLocation) "0, 0, 0" 1.0 1.0 0.0 0 0 0 0))

(fn ConstructionScript)