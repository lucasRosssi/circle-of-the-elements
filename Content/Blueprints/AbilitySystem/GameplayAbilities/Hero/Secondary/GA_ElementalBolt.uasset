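; GA_ElementalBolt is a hero secondary gameplay ability for a projectile bolt that changes with the consumed Elemental Flow element.
; On consuming flow, it looks up the element tag in two maps to add that element's status effect and override the projectile class.
; Once flow is consumed, it clears the added status effects but leaves the projectile override set.
; Activation defers to the parent ability, and the tag switches drive no logic.
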(event Ability|EventActivateAbility
  (|CallParentFunction))

(event EventOnElementalFlowConsumed
  (params (ElementalFlowTag :type Gameplay%20Tag%20Structure%20%28by%20ref%29))
  (Utilities|Array|Clear (Variables|Default|GetAdditionalStatusEffectData)))

(event EventOnConsumeElementalFlow
  (params (ElementalFlowTag :type Gameplay%20Tag%20Structure%20%28by%20ref%29))
  (Utilities|Array|Add (Variables|Default|GetAdditionalStatusEffectData) (.Value (Utilities|Map|Find (Variables|Default|GetElementsStatusEffects) ElementalFlowTag)))
  (Variables|Default|SetOverrideProjectileClass (.Value (Utilities|Map|Find (Variables|Default|GetElementsProjectiles) ElementalFlowTag)))
  (|SwitchGameplayTag ElementalFlowTag))