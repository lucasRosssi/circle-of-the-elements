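; Vilkar's primary hero gameplay ability, which leaves activation and end handling to its parent class.
; When Elemental Flow is invoked, it looks up the element's gameplay tag in ElementsStatusEffects and adds that entry to AdditionalStatusEffectData.
; Once the flow is used, it clears that data.
; Both flow handlers end in a gameplay tag switch with no per-element logic attached.
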(event Ability|EventActivateAbility
  (|CallParentFunction))

(event EventOnElementalFlowUsed
  (params (ElementalFlowTag :type Gameplay%20Tag%20Structure%20%28by%20ref%29))
  (Utilities|Array|Clear (Variables|Default|GetAdditionalStatusEffectData))
  (|SwitchGameplayTag ElementalFlowTag))

(event EventOnUseElementalFlow
  (params (ElementalFlowTag :type Gameplay%20Tag%20Structure%20%28by%20ref%29))
  (Utilities|Array|Add (Variables|Default|GetAdditionalStatusEffectData) (.Value (Utilities|Map|Find (Variables|Default|GetElementsStatusEffects) ElementalFlowTag)))
  (|SwitchGameplayTag ElementalFlowTag))

(event Ability|EventOnEndAbility
  (params (bWasCancelled :type Boolean))
  (|CallParentFunction bWasCancelled))