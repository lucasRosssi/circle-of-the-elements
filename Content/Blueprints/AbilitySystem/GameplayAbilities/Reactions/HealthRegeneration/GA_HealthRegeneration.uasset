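; Gameplay ability that heals its owning actor when an encounter finishes.
; On activation it binds to the encounter manager's finished delegate and waits for the Respite passive's gameplay event, which sets a bonus flag.
; At encounter end it reads a float attribute as the base heal and self-applies GE_Heal, doubling the amount and clearing the flag if the bonus is pending.
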(event Custom|OnEncounterFinish
  (CallFunction|ApplyHealing (.ReturnValue (Ability|Attribute|GetFloatAttribute (Ability|GetAvatarActorfromActorInfo) "(AttributeName=\"HealthRegeneration\",Attribute=/Script/Aura.AuraAttributeSet:HealthRegeneration,AttributeOwner=/Script/CoreUObject.Class'\"/Script/Aura.AuraAttributeSet\"')"))))

(event Ability|EventActivateAbility
  (EventDispatchers|BindEventtoOnEncounterFinishedDelegate (Class|AuraSystemsLibrary|GetEncounterManager) (EventDispatchers|CreateEvent :!event Custom|OnEncounterFinish))
  (Ability|Tasks|WaitGameplayEvent "(TagName=\"Abilities.Passive.Common.Respite\")" 0
    (:EventReceived
      (Variables|Default|SetApplyExtraHeal true))))

(fn ApplyHealing
  (params (BaseHeal :type Float%20%28single-precision%29))
  (bind _returnvalue (Ability|GetAbilitySystemComponentfromActorInfo))
  (bind _returnvalue_2 (Ability|GetAbilitySystemComponentfromActorInfo))
  (if (Variables|Default|GetApplyExtraHeal)
    (Class|AuraAbilitySystemLibrary|ApplyAbilityEffect (Utilities|Struct|MakeAbilityParams (Ability|GetAvatarActorfromActorInfo) _returnvalue_2 _returnvalue_2 1 "(DamageEffectClass=None,DamageType=(TagName=\"\"),BaseDamage=0.000000,bApplyHitReact=False)" (Utilities|Struct|MakeHealParams "/Game/Blueprints/AbilitySystem/GameplayEffects/GE_Heal.GE_Heal_C" (* 2.0 BaseHeal))))
    (Variables|Default|SetApplyExtraHeal false)
    (else
      (Class|AuraAbilitySystemLibrary|ApplyAbilityEffect (Utilities|Struct|MakeAbilityParams (Ability|GetAvatarActorfromActorInfo) _returnvalue _returnvalue 1 "(DamageEffectClass=None,DamageType=(TagName=\"\"),BaseDamage=0.000000,bApplyHitReact=False)" (Utilities|Struct|MakeHealParams "/Game/Blueprints/AbilitySystem/GameplayEffects/GE_Heal.GE_Heal_C" BaseHeal))))))