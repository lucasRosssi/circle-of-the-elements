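; GA_Shock is a gameplay ability for the shock reaction that paralyzes its owner.
; On activation it applies the SE_Paralysis gameplay effect to the owner through the Paralyze event and starts a looping timer with a short interval.
; The ability never ends itself in this graph, and OnEndAbility clears and invalidates the stored timer handle.
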(event Custom|Paralyze
  (Ability|ApplyGameplayEffectToOwner "/Game/Blueprints/AbilitySystem/GameplayEffects/StatusEffects/Incapacitations/SE_Paralysis.SE_Paralysis_C"))

(event Ability|EventActivateAbility
  (CallFunction|Paralyze)
  (bind _returnvalue (Utilities|Time|SetTimerbyEvent (EventDispatchers|CreateEvent :!event Custom|Paralyze) 1.5 true))
  (Variables|Default|SetTimerHandle _returnvalue))

(event Ability|EventOnEndAbility
  (params (bWasCancelled :type Boolean))
  (bind _timerhandle (Variables|Default|GetTimerHandle))
  (if (Utilities|Time|IsValidTimerHandle _timerhandle)
    (Utilities|Time|ClearandInvalidateTimerbyHandle _timerhandle)))