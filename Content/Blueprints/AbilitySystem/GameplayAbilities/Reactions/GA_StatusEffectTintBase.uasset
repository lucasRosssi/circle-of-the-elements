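; Base gameplay ability that tints the avatar's mesh to show a status effect.
; On activation it creates a dynamic material instance for each mesh material and sets its MaterialTint parameter to Tint.
; With TintStacks on, it watches the first active effect matching StatusAssetTags and multiplies the tint by the new stack count.
; With RemoveTintOnEnd on, ending the ability zeroes the tint parameter.
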(event Ability|EventActivateAbility
  (bind _returnvalue (Class|CombatInterface|GetAvatarMesh(Message) (Ability|GetAvatarActorfromActorInfo)))
  (CallFunction|CreateDynamicandApplyTint _returnvalue 1)
  (if (Variables|Default|GetTintStacks)
    (bind _returnvalue_2 (GameplayEffects|GetActiveEffectswithAllTags (Ability|GetAbilitySystemComponentfromActorInfo) (Variables|Default|GetStatusAssetTags)))
    (bind _newcount (|WaitforGameplayEffectStackChange (Utilities|Array|Get(acopy) _returnvalue_2))
      (:OnChange
        (CallFunction|ApplyTint _newcount)))))

(event Ability|EventOnEndAbility
  (params (bWasCancelled :type Boolean))
  (if (Variables|Default|GetRemoveTintOnEnd)
    (CallFunction|ApplyTint)))

(fn CreateDynamicandApplyTint
  (params (Mesh :type Skeletal%20Mesh%20Component%20Object%20Reference) (Stacks :type Integer))
  (bind _returnvalue (Math|Conversions|ToFloat(Integer) Stacks))
  (for _index (range 0 (- (Rendering|Material|GetNumMaterials Mesh) 1))
    (bind _returnvalue_2 (Rendering|Material|CreateDynamicMaterialInstance Mesh _index (Rendering|Material|GetMaterial Mesh _index) "None" :!class /Script/Engine.PrimitiveComponent))
    (Utilities|Array|Add (Variables|Default|GetDynamicInstances) _returnvalue_2)
    (Rendering|Material|SetVectorParameterValue _returnvalue_2 "MaterialTint" (* (Variables|Default|GetTint) (Utilities|Struct|MakeLinearColor _returnvalue _returnvalue _returnvalue _returnvalue)) :!class /Script/Engine.MaterialInstanceDynamic))
  (return))

(fn ApplyTint
  (params (Stacks :type Integer))
  (bind _dynamicinstances (Variables|Default|GetDynamicInstances))
  (bind _returnvalue (Math|Conversions|ToFloat(Integer) Stacks))
  (for _index (range 0 (- (Utilities|Array|Length _dynamicinstances) 1))
    (Rendering|Material|SetVectorParameterValue (Utilities|Array|Get(acopy) _dynamicinstances _index) "MaterialTint" (* (Variables|Default|GetTint) (Utilities|Struct|MakeLinearColor _returnvalue _returnvalue _returnvalue _returnvalue)) :!class /Script/Engine.MaterialInstanceDynamic))
  (return))