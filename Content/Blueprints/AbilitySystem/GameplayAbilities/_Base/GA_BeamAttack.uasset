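; Base gameplay ability for a channeled beam attack aimed at the mouse hit, running until input release, montage interruption or failed cost.
; After the montage's spawn event, a looping timer retraces the first target, rebuilding beam gameplay cues and optional ricochet chains when it changes.
; Ticks apply per-hit-adjusted effects to cued actors and commit cost on the server.
; Ending clears cues and commits cooldown if the beam fired.
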(event Custom|OnFirstTargetChanged
  (CallFunction|RemoveBeamCuesfromAllTargets)
  (Class|ActiveAbility|ClearRicochetHitTargets)
  (GameplayCue|RemoveGameplayCue (Variables|AbilityDefaults|Beam|GetGameplayCueBeamLoop)))

(event Custom|ApplyAbilityEffectEachPeriod
  (bind _datahandle (|TargetData)
    (:ValidData
      (CallFunction|HandleHitResult _datahandle)
      (Class|BeamAbility|TraceFirstTarget (Variables|Default|GetMouseHitLocation))
      ;[1 1 1] Check if the first hit target changed
      (if (!= (Variables|Default|GetFirstTarget) (Variables|Default|GetMouseHitActor))
        (Default|CallFirstTargetChanged)
        ;[1 0.2281 0.2281] If changed, recalculate the gameplay cues and targets, before applying effects
        (CallFunction|TargetBeamtoFirstTarget)
        (if (Utilities|Enum|Equal(Enum) (Variables|Default|GetRangedHitMode) "Ricochet")
          (CallFunction|BounceBeamtoAdditionalTargets)
          (CallFunction|CommitBeamEffect :!label _label)
          (CallFunction|HandleResources))
        (else
          (goto _label))))))

(event Ability|EventActivateAbility
  (EventDispatchers|BindEventtoFirstTargetChanged (EventDispatchers|CreateEvent :!event Custom|OnFirstTargetChanged))
  (bind _datahandle (|TargetData)
    (:ValidData
      (CallFunction|HandleHitResult _datahandle)
      (|PlayMontageandWaitProxy "None" (Variables|Default|GetMontageToPlay) (Class|ActiveAbility|GetMontagePlayRate) "None" true (Class|ActiveAbility|GetAnimRootMotionTranslateScale) 0.0 false
        (:then
          (Ability|Tasks|WaitInputRelease false
            (:then
              (Ability|Tasks|WaitGameplayEvent "(TagName=\"Event.Montage.SpawnProjectile\")" 0
                (:EventReceived
                  (GameplayCue|ExecuteGameplayCue :GameplayCueTag (Variables|AbilityDefaults|Beam|GetGameplayCueOnOwner))
                  (bind _returnvalue (Utilities|Time|SetTimerbyEvent (delegate Custom|ApplyAbilityEffectEachPeriod) (Variables|Default|GetBeamTickPeriod) true))
                  (Variables|Default|SetBeamTickTimerHandle _returnvalue)
                  (Variables|Default|SetCanCommitCooldown true))))
            (:OnRelease
              (Ability|EndAbility :!label _label))))
        (:OnInterrupted
          (goto _label))
        (:OnCancelled
          (goto _label))))))

(event Ability|EventOnEndAbility
  (params (bWasCancelled :type Boolean))
  (GameplayCue|RemoveGameplayCue (Variables|AbilityDefaults|Beam|GetGameplayCueOnOwner))
  (GameplayCue|RemoveGameplayCue (Variables|AbilityDefaults|Beam|GetGameplayCueBeamLoop))
  (CallFunction|RemoveBeamCuesfromAllTargets)
  (EventDispatchers|UnbindallEventsfromFirstTargetChanged)
  (CallFunction|HandleCooldown)
  (CallFunction|ResetVariables))

(fn BounceBeamtoAdditionalTargets
  (Utilities|FlowControl|ForLoopwithBreak 1 (- (Class|ActiveAbility|GetMaxHitCount) 1) :!label _label
    (:LoopBody
      (bind _returnvalue (Class|ActiveAbility|GetNextRicochetTarget (Variables|Default|GetHitTarget)))
      (Utilities|IsValid _returnvalue
        (:Is%20Valid
          (Variables|Default|SetNextTarget _returnvalue)
          (GameplayCue|AddGameplayCueOnActor(Looping) (Variables|Default|GetNextTarget) (Variables|AbilityDefaults|Beam|GetGameplayCueBeamLoop) (Ability|GameplayCue|MakeGameplayCueParameters :Location (Transformation|GetActorLocation (Variables|Default|GetNextTarget)) :SourceObject (Variables|Default|GetNextTarget) :AbilityLevel (Variables|Default|GetSocketIndex) :TargetAttachComponent (Variables|/Script/Engine.Actor|GetRootComponent (Variables|Default|GetHitTarget))))
          (Utilities|Map|Add :TargetMap (Variables|Default|GetCueParamsArray) :Key (Variables|Default|GetNextTarget))
          (Variables|Default|SetHitTarget (Variables|Default|GetNextTarget)))
        (:Is%20Not%20Valid
          (goto _label Break))))
    (:Completed
      (return))))

(fn TargetBeamtoFirstTarget
  (bind _mousehitactor (Variables|Default|GetMouseHitActor))
  (bind _mousehitactor_2 (Variables|Default|GetMouseHitActor))
  (Variables|Default|SetFirstTargetCueParams (Ability|GameplayCue|MakeGameplayCueParameters :Location (Variables|Default|GetMouseHitLocation) :SourceObject (Variables|Default|GetMouseHitActor) :AbilityLevel (Variables|Default|GetSocketIndex) :TargetAttachComponent (Class|BeamAbility|GetComponenttoAttachGameplayCue)))
  ;[1 1 1] Hit an enemy?
  (if (Class|AuraAbilitySystemLibrary|AreActorsEnemies (Ability|GetAvatarActorfromActorInfo) (Variables|Default|GetMouseHitActor))
    (Variables|Default|SetFirstTarget _mousehitactor)
    (Variables|Default|SetHitTarget _mousehitactor)
    (GameplayCue|AddGameplayCueOnActor(Looping) (Variables|Default|GetFirstTarget) (Variables|AbilityDefaults|Beam|GetGameplayCueBeamLoop) (Variables|Default|GetFirstTargetCueParams))
    (Utilities|Map|Add (Variables|Default|GetCueParamsArray) (Variables|Default|GetFirstTarget) (Variables|Default|GetFirstTargetCueParams))
    (else
      (GameplayCue|AddGameplayCueOnActor(Looping) (Ability|GetAvatarActorfromActorInfo) (Variables|AbilityDefaults|Beam|GetGameplayCueBeamLoop) (Variables|Default|GetFirstTargetCueParams))
      (Variables|Default|SetFirstTarget _mousehitactor_2)
      (Variables|Default|SetHitTarget _mousehitactor_2))))

(fn RemoveBeamCuesfromAllTargets
  (bind _keys (Utilities|Map|Keys (Variables|Default|GetCueParamsArray)))
  (for _array_element _keys
    (if (.ReturnValue (Utilities|Map|Find (Variables|Default|GetCueParamsArray) _array_element))
      (GameplayCue|RemoveGameplayCueOnActor(Looping) _array_element (Variables|AbilityDefaults|Beam|GetGameplayCueBeamLoop) (.Value (Utilities|Map|Find (Variables|Default|GetCueParamsArray) _array_element)))))
  (Utilities|Map|Clear (Variables|Default|GetCueParamsArray))
  (return))

(fn CommitBeamEffect
  (if (Utilities|DoesObjectImplementInterface (Variables|Default|GetFirstTarget) "/Script/Aura.CombatInterface")
    (Ability|HasAuthority
      (:True
        (bind _keys (Utilities|Map|Keys (Variables|Default|GetCueParamsArray)))
        (for (_array_element _array_index) _keys
          (bind _returnvalue (Class|ActiveDamageAbility|ApplyEffectChangePerHittoAbilityParams (Class|BaseAbility|MakeAbilityParamsfromDefaults _array_element) _array_index))
          (Class|AuraAbilitySystemLibrary|ApplyAbilityEffect _returnvalue))))
    (else
      (CallFunction|HandleEnvironmentHit))))

(fn HandleHitResult
  (params (HitResult :type Gameplay%20Ability%20Target%20Data%20Handle%20Structure%20%28by%20ref%29))
  (bind _returnvalue (Ability|TargetData|GetHitResultfromTargetData HitResult))
  (Class|CombatInterface|UpdateFacingTarget(Message) (Ability|GetAvatarActorfromActorInfo) (.Location (Collision|BreakHitResult _returnvalue)))
  (Class|BeamAbility|StoreMouseDataInfo _returnvalue))

(fn HandleResources
  (Ability|HasAuthority
    (:True
      (bind _returnvalue (Ability|CommitAbilityCost false))
      (if (not _returnvalue)
        (Ability|EndAbility)))))

(fn HandleEnvironmentHit
  (GameplayCue|RemoveGameplayCue (Variables|AbilityDefaults|Beam|GetGameplayCueBeamLoop))
  (GameplayCue|AddGameplayCueOnActor(Looping) (Ability|GetAvatarActorfromActorInfo) (Variables|AbilityDefaults|Beam|GetGameplayCueBeamLoop) (Ability|GameplayCue|MakeGameplayCueParameters :Location (Variables|Default|GetMouseHitLocation) :SourceObject (Variables|Default|GetMouseHitActor) :TargetAttachComponent (Class|BeamAbility|GetComponenttoAttachGameplayCue))))

(fn HandleCooldown
  (Ability|HasAuthority
    (:True
      (if (Variables|Default|GetCanCommitCooldown)
        (Ability|CommitAbilityCooldown false)
        (Variables|Default|SetCanCommitCooldown false)))))

(fn ResetVariables
  (Variables|Default|SetFirstTargetCueParams "")
  (Variables|Default|SetFirstTarget 0)
  (Variables|Default|SetHitTarget 0)
  (Variables|Default|SetNextTarget 0))