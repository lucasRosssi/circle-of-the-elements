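; Base area-attack gameplay ability that damages living enemies within a radius of a chosen origin.
; Players aim with a targeting actor and confirm or cancel, while AI uses its combat target's location.
; Both paths face the origin and play a montage, whose SpawnProjectile event fires the burst GameplayCue and applies effects.
; The ability commits only after applying effects, and damage always targets Enemies, whereas the targeting display uses AbilityTargetTeam.
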(event Custom|Event%20TargetSet
  (if (Variables|Default|GetbIsPlayerAbility)
    ;[0.6106 0.2968 1] Effective State
    (bind _datahandle (|TargetData)
      (:ValidData
        (bind _output_get (Variables|Default|SetAreaOrigin (.ImpactPoint (Collision|BreakHitResult (Ability|TargetData|GetHitResultfromTargetData _datahandle)))))
        (Class|CombatInterface|UpdateFacingTarget(Message) (Ability|GetAvatarActorfromActorInfo) _output_get)))
    (else
      ;;[1 0 0.1516] AI Targeting
      (bind _returnvalue (Class|CombatInterface|GetCombatTarget(Message) (Ability|GetAvatarActorfromActorInfo)))
      (bind _output_get_2 (Variables|Default|SetAreaOrigin (Transformation|GetActorLocation _returnvalue)))
      (Class|CombatInterface|UpdateFacingTarget(Message) (Ability|GetAvatarActorfromActorInfo) _output_get_2)))
  (|PlayMontageandWaitProxy "None" (Variables|Default|GetMontageToPlay) (Class|ActiveAbility|GetMontagePlayRate) "None" true (Class|ActiveAbility|GetAnimRootMotionTranslateScale) 0.0
    (:then
      (Ability|Tasks|WaitGameplayEvent "(TagName=\"Event.Montage.SpawnProjectile\")" 0
        (:EventReceived
          (Class|GameplayAbility|ExecuteGameplayCuewithParams (Variables|Default|GetAreaBurstGC) (Ability|GameplayCue|MakeGameplayCueParameters :NormalizedMagnitude (Class|BaseAbility|GetAreaRadius) :Location (Variables|Default|GetAreaOrigin)))
          (CallFunction|ApplyDamagetoArea))))
    (:OnCompleted
      (Ability|EndAbility :!label _label))
    (:OnBlendOut
      (goto _label))
    (:OnInterrupted
      (goto _label))
    (:OnCancelled
      (goto _label))))

(event Ability|EventActivateAbility
  (if (Variables|Default|GetbIsPlayerAbility)
    (EventDispatchers|BindEventtoTargetSet (delegate Custom|Event%20TargetSet))
    ;[1 1 1] Targeting State
    (Class|PlayerInterface|ShowTargetingActor(Message) (Ability|GetAvatarActorfromActorInfo) (Variables|Default|GetTargetingActorClass) (Variables|Default|GetAbilityTargetTeam) (Class|BaseAbility|GetAreaRadius))
    (|WaitConfirmCancel
      (:OnConfirm
        (Default|CallTargetSet))
      (:OnCancel
        (Ability|EndAbility)))
    (Class|PlayerInterface|HideTargetingActor(Message) (Ability|GetAvatarActorfromActorInfo))
    (else
      (Default|CallTargetSet))))

(event Ability|EventOnEndAbility
  (params (bWasCancelled :type Boolean))
  (Class|PlayerInterface|HideTargetingActor(Message) (Ability|GetAvatarActorfromActorInfo)))

(fn ApplyDamagetoArea
  (bind _outoverlappingactors (Class|AuraAbilitySystemLibrary|GetAliveCharactersWithinRadius (Ability|GetAvatarActorfromActorInfo) (Utilities|Array|MakeArray 0) (Class|BaseAbility|GetAreaRadius) (Variables|Default|GetAreaOrigin) "Enemies"))
  (for _array_element _outoverlappingactors
    (Class|AuraAbilitySystemLibrary|ApplyAbilityEffect (Class|BaseAbility|MakeAbilityParamsfromDefaults _array_element)))
  (Ability|CommitAbility)
  (Ability|EndAbility))