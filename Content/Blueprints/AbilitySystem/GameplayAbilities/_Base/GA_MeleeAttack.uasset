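; Base melee attack ability with montage-driven combo sequences, shared by players and AI.
; Each step turns the player toward the mouse target or AI toward its combat target, then plays the montage.
; Montage gameplay events open the combo window for input, start its closing timer, and trigger either weapon collision or attack scans.
; The ability ends on window timeout, montage completion, cancellation or final-step blend out, and commits in OnEndAbility.
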(event Custom|ComboWindowEnd
  (Variables|Default|SetbInComboWindow false)
  (Ability|EndAbility))

(event Ability|EventActivateAbility
  (bind (_montage _playrate _rootmotionscale) (Class|ActiveAbility|GetMontageParams))
  (if (Variables|Default|GetbIsPlayerAbility)
    (bind _datahandle (|TargetDataUnderMouse)
      (:ValidData
        (CallFunction|FacetoTarget _datahandle)))
    (else
      (CallFunction|GetAITargetData)))
  (|PlayMontageandWaitProxy "None" _montage _playrate "None" true _rootmotionscale 0.0 false
    (:then
      (Ability|Tasks|WaitInputPress false
        (:then
          (Ability|Tasks|WaitGameplayEvent "(TagName=\"Event.Montage.ComboStart\")" 0 true
            (:then
              (Ability|Tasks|WaitGameplayEvent "(TagName=\"Event.Montage.ComboEnd\")" 0 true
                (:then
                  ;[1 0.2406 0.2406] Handle Melee Impact
                  (if (Utilities|Enum|Equal(Enum) (Class|MeleeAttackAbility|GetMeleeHitMode) "Weapon")
                    (Ability|Tasks|WaitGameplayEvent "(TagName=\"Event.Montage.WeaponCollisionStart\")" 0
                      (:EventReceived
                        (Class|MeleeAttackAbility|HandleWeaponCollision)
                        (Ability|Tasks|WaitGameplayEvent "(TagName=\"Event.Montage.WeaponCollisionEnd\")" 0
                          (:EventReceived
                            (CallFunction|StopWeaponCollision)))))
                    (else
                      (Ability|Tasks|WaitGameplayEvent "(TagName=\"Event.Montage.AttackScan\")" 0
                        (:EventReceived
                          (Class|MeleeAttackAbility|ExecuteAttackScan))))))
                (:EventReceived
                  (bind _returnvalue (Utilities|Time|SetTimerbyEvent (delegate Custom|ComboWindowEnd) (Variables|Default|GetComboWindowEndTime)))
                  (Variables|Default|SetComboWindowEndTimerHandle _returnvalue))))
            (:EventReceived
              (Variables|Default|SetbInComboWindow true)
              (Class|ActiveDamageAbility|HandleComboSequence))))
        (:OnPress
          (Variables|Default|SetbComboInputPressed true)
          (Class|ActiveDamageAbility|HandleComboSequence))))
    (:OnCompleted
      (Ability|EndAbility :!label _label))
    (:OnBlendOut
      (if (CallFunction|IsLastSequence)
        (Ability|EndAbility)))
    (:OnCancelled
      (goto _label))))

(event Ability|EventOnEndAbility
  (params (bWasCancelled :type Boolean))
  (if (Utilities|Enum|Equal(Enum) (Variables|Default|GetMeleeHitMode) "Weapon")
    (CallFunction|StopWeaponCollision))
  (Ability|CommitAbility))

(event EventOnNextComboSequence
  (bind (_montage _playrate _rootmotionscale) (Class|ActiveAbility|GetMontageParams))
  (if (Utilities|Time|IsValidTimerHandle (Variables|Default|GetComboWindowEndTimerHandle))
    (Utilities|Time|ClearandInvalidateTimerbyHandle (Variables|Default|GetComboWindowEndTimerHandle)))
  (if (Variables|Default|GetbIsPlayerAbility)
    (bind _datahandle (|TargetDataUnderMouse)
      (:ValidData
        (CallFunction|FacetoTarget _datahandle)))
    (else
      (CallFunction|GetAITargetData)))
  (|PlayMontageandWaitProxy "None" _montage _playrate "None" true _rootmotionscale 0.0 false
    (:then
      (Ability|Tasks|WaitInputPress false
        (:then
          (Ability|Tasks|WaitGameplayEvent "(TagName=\"Event.Montage.ComboStart\")" 0 true
            (:then
              (Ability|Tasks|WaitGameplayEvent "(TagName=\"Event.Montage.ComboEnd\")" 0 true
                (:then
                  ;[1 0.2406 0.2406] Handle Melee Impact
                  (if (Utilities|Enum|Equal(Enum) (Class|MeleeAttackAbility|GetMeleeHitMode) "Weapon")
                    (Ability|Tasks|WaitGameplayEvent "(TagName=\"Event.Montage.WeaponCollisionStart\")" 0
                      (:EventReceived
                        (Class|MeleeAttackAbility|HandleWeaponCollision)
                        (Ability|Tasks|WaitGameplayEvent "(TagName=\"Event.Montage.WeaponCollisionEnd\")" 0
                          (:EventReceived
                            (CallFunction|StopWeaponCollision)))))
                    (else
                      (Ability|Tasks|WaitGameplayEvent "(TagName=\"Event.Montage.AttackScan\")" 0
                        (:EventReceived
                          (Class|MeleeAttackAbility|ExecuteAttackScan))))))
                (:EventReceived
                  (bind _returnvalue (Utilities|Time|SetTimerbyEvent (delegate Custom|ComboWindowEnd) (Variables|Default|GetComboWindowEndTime)))
                  (Variables|Default|SetComboWindowEndTimerHandle _returnvalue))))
            (:EventReceived
              (Variables|Default|SetbInComboWindow true)
              (Class|ActiveDamageAbility|HandleComboSequence))))
        (:OnPress
          (Variables|Default|SetbComboInputPressed true)
          (Class|ActiveDamageAbility|HandleComboSequence))))
    (:OnCompleted
      (Ability|EndAbility :!label _label))
    (:OnBlendOut
      (if (CallFunction|IsLastSequence)
        (Ability|EndAbility)))
    (:OnCancelled
      (goto _label))))

(fn GetAITargetData
  (bind _returnvalue (Ability|GetAvatarActorfromActorInfo))
  (bind _returnvalue_2 (Class|CombatInterface|GetCombatTarget(Message) _returnvalue))
  (Class|CombatInterface|UpdateFacingTarget(Message) _returnvalue (Transformation|GetActorLocation _returnvalue_2)))

(fn StopWeaponCollision
  (bind _returnvalue (Class|CombatInterface|EnableWeaponCollision(Message) (Ability|GetAvatarActorfromActorInfo) false))
  (EventDispatchers|UnbindallEventsfromOnComponentBeginOverlap _returnvalue))

(fn FacetoTarget
  (params (HitResult :type Gameplay%20Ability%20Target%20Data%20Handle%20Structure%20%28by%20ref%29))
  (Class|CombatInterface|UpdateFacingTarget(Message) (Ability|GetAvatarActorfromActorInfo) (.Location (Collision|BreakHitResult (Ability|TargetData|GetHitResultfromTargetData HitResult)))))

(fn IsLastSequence
  (return (>= (Variables|Default|GetComboIndex) (- (Utilities|Array|Length (Variables|Default|GetComboSequenceData)) 1))))