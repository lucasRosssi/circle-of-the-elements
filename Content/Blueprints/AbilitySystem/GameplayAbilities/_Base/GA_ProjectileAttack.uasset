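; Base gameplay ability for projectile attacks, aiming players at target data under the mouse and non-player avatars at their combat target.
; A montage drives timing, with gameplay events attaching a held-projectile Niagara effect, then triggering default single-shot or channeling mode.
; Channeling loops on a timer, rechecking cost, cooldown and mouse target until input release or failed checks.
; Each shot spawns a projectile and commits the ability only with authority.
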(event Custom|ChannelingLoop
  (if (CallFunction|CheckActivatable)
    (bind _datahandle (|TargetDataUnderMouse)
      (:ValidData
        (Class|CombatInterface|UpdateFacingTarget(Message) (Ability|GetAvatarActorfromActorInfo) (CallFunction|GetLocationfromTargetData _datahandle))
        (CallFunction|SpawnProjectileandCommit)))
    (else
      (Ability|EndAbility))))

(event Custom|Default_Event
  (CallFunction|SpawnProjectileandCommit))

(event Custom|Channeling_Event
  (bind _returnvalue (Utilities|Time|SetTimerbyEvent (delegate Custom|ChannelingLoop) (Variables|Default|GetChannelingTick) true))
  (Variables|Default|SetChannelingTimerHandle _returnvalue)
  (Ability|Tasks|WaitInputRelease false
    (:OnRelease
      (Ability|EndAbility))))

(event Ability|EventActivateAbility
  (bind _returnvalue (Ability|GetAvatarActorfromActorInfo))
  (if (Variables|Default|GetbIsPlayerAbility)
    (bind _datahandle (|TargetDataUnderMouse)
      (:ValidData
        (Class|CombatInterface|UpdateFacingTarget(Message) (Ability|GetAvatarActorfromActorInfo) (CallFunction|GetLocationfromTargetData _datahandle))))
    (else
      (bind _returnvalue_2 (Class|CombatInterface|GetCombatTarget(Message) _returnvalue))
      (Class|CombatInterface|UpdateFacingTarget(Message) _returnvalue (Transformation|GetActorLocation _returnvalue_2))
      (Variables|Default|SetTargetLocation (Transformation|GetActorLocation _returnvalue_2))))
  (|PlayMontageandWaitProxy "None" (Variables|Default|GetMontageToPlay) (Class|ActiveAbility|GetMontagePlayRate) "None" true (Class|ActiveAbility|GetAnimRootMotionTranslateScale) 0.0 false
    (:then
      (Ability|Tasks|WaitGameplayEvent "(TagName=\"Event.Montage.HoldProjectile\")" 0
        (:then
          (Ability|Tasks|WaitGameplayEvent "(TagName=\"Event.Montage.SpawnProjectile\")" 0
            (:EventReceived
              (Utilities|IsValid (Variables|Default|GetHoldingProjectile)
                (:Is%20Valid
                  (Components|Activation|Deactivate (Variables|Default|GetHoldingProjectile)))
                (:Is%20Not%20Valid
                  _))
              (switch Utilities|FlowControl|Switch|SwitchonEAbilityActivationMode (Variables|Default|GetActivationMode)
                (:Default
                  (CallFunction|DefaultEvent))
                (:Channeling
                  (CallFunction|ChannelingEvent))))))
        (:EventReceived
          (bind _returnvalue_3 (Niagara|SpawnSystemAttached (Variables|Default|GetHoldingNiagara) (Class|GameplayAbility|GetOwningComponentfromActorInfo) (Variables|Default|GetAbilitySocketName) "0, 0, 0" "0, 0, 0" "KeepRelativeOffset" false))
          (Variables|Default|SetHoldingProjectile _returnvalue_3))))
    (:OnCompleted
      (Utilities|IsValid (Variables|Default|GetHoldingProjectile) :!label _label
        (:Is%20Valid
          (Components|Activation|Deactivate (Variables|Default|GetHoldingProjectile)))
        (:Is%20Not%20Valid
          _))
      (Ability|EndAbility))
    (:OnBlendOut
      (goto _label))
    (:OnInterrupted
      (goto _label))
    (:OnCancelled
      (goto _label))))

(event Ability|EventOnEndAbility
  (params (bWasCancelled :type Boolean))
  (bind _channelingtimerhandle (Variables|Default|GetChannelingTimerHandle))
  (if (Utilities|Time|IsValidTimerHandle _channelingtimerhandle)
    (Utilities|Time|ClearandInvalidateTimerbyHandle _channelingtimerhandle)))

(fn CheckActivatable
  (bind _returnvalue (Class|GameplayAbility|CheckAbilityCooldown))
  (bind _returnvalue_2 (Class|GameplayAbility|CheckAbilityCost))
  (return (and _returnvalue_2 _returnvalue)))

(fn SpawnProjectileandCommit
  (Class|ProjectileAbility|SpawnProjectile (Variables|Default|GetTargetLocation) (Variables|Default|GetAbilitySocketName) (Variables|Default|GetbUseWeaponSocket))
  (Ability|HasAuthority
    (:True
      (Ability|CommitAbility))))

(fn GetLocationfromTargetData
  (params (TargetData :type Gameplay%20Ability%20Target%20Data%20Handle%20Structure%20%28by%20ref%29))
  (return (.Location (Collision|BreakHitResult (Ability|TargetData|GetHitResultfromTargetData TargetData)))))