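; Gameplay ability for the goblin's spear melee attack.
; On activation it turns the avatar toward its combat target and plays the spear attack montage, ending the ability when the montage completes, is interrupted or is cancelled.
; An AttackScan montage event triggers a small sphere check at the weapon's tip socket, damaging living characters in range that are enemies of the attacker.
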(event Ability|EventActivateAbility
  (bind _returnvalue (Ability|GetAvatarActorfromActorInfo))
  (bind _returnvalue_2 (Ability|GetAvatarActorfromActorInfo))
  (bind _returnvalue_3 (Class|CombatInterface|GetCombatTarget(Message) _returnvalue))
  (Class|CombatInterface|UpdateFacingTarget(Message) _returnvalue (Transformation|GetActorLocation _returnvalue_3))
  (|PlayMontageandWaitProxy "None" "/Game/Assets/Enemies/Goblin/Animations/Spear/AM_Attack_Spear.AM_Attack_Spear" 1.0 "None" true 1.0 0.0
    (:then
      (Ability|Tasks|WaitGameplayEvent "(TagName=\"Event.Montage.AttackScan\")" 0
        (:EventReceived
          (bind _returnvalue_4 (Class|CombatInterface|GetAbilitySocketLocation(Message) _returnvalue_2 "TipSocket" true))
          (bind _outoverlappingactors (Class|AuraAbilitySystemLibrary|GetAliveCharactersWithinRadius _returnvalue_2 (Utilities|Array|MakeArray _returnvalue_2) 2e+01 _returnvalue_4))
          (for _array_element _outoverlappingactors
            (if (Class|AuraAbilitySystemLibrary|AreActorsEnemies (Ability|GetAvatarActorfromActorInfo) _array_element)
              (Class|AuraDamageGameplayAbility|CauseDamage _array_element))))))
    (:OnCompleted
      (Ability|EndAbility :!label _label))
    (:OnInterrupted
      (goto _label))
    (:OnCancelled
      (goto _label))))