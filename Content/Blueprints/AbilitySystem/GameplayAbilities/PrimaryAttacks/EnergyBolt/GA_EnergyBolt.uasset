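; Gameplay ability for the Energy Bolt primary attack, which casts a projectile at the location under the mouse cursor.
; A target data task supplies the hit location, which is stored and sent to the avatar as its facing target.
; The cast montage then plays, and its gameplay event triggers the projectile spawn from the weapon's tip socket.
; The ability ends when the montage completes, blends out, is interrupted or is cancelled.
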(event Ability|EventActivateAbility
  (bind _datahandle (|TargetDataUnderMouse)
    (:ValidData
      (Variables|Default|SetProjectileTargetLocation (.Location (Collision|BreakHitResult (Ability|TargetData|GetHitResultfromTargetData _datahandle))))
      (Class|CombatInterface|UpdateFacingTarget(Message) (Ability|GetAvatarActorfromActorInfo) (Variables|Default|GetProjectileTargetLocation))
      (|PlayMontageandWaitProxy "None" "/Game/Assets/Characters/Aura/Animations/Abilities/AM_Cast_EnergyBolt.AM_Cast_EnergyBolt" 0.8 "None" true 1.0 0.0
        (:then
          (Ability|Tasks|WaitGameplayEvent "(TagName=\"Event.Montage.SpawnProjectile\")" 0
            (:EventReceived
              (Class|ProjectileSpell|SpawnProjectile (Variables|Default|GetProjectileTargetLocation) "TipSocket" true))))
        (:OnCompleted
          (Ability|EndAbility :!label _label))
        (:OnBlendOut
          (goto _label))
        (:OnInterrupted
          (goto _label))
        (:OnCancelled
          (goto _label))))))